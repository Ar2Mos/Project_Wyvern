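; Floating battle number actor that displays initiative loss, healing or MP restoration as coloured, rising text.
; The construction script formats the value, picks its colour and sets projectile velocity for the drift.
; A damage branch with random drift and enlarged red criticals sits behind a constant-true condition, so it never runs.
; BeginPlay retries until it caches the player's view target, and Tick rotates the actor relative to it.
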(event EventBeginPlay
  (bind _output_get (Variables|Default|SetCameraReference (Pawn|GetViewTarget (Game|GetPlayerController 0)) :!label _label))
  (Utilities|IsValid _output_get
    (:Is%20Not%20Valid
      (Utilities|FlowControl|Delay 0.2)
      (goto _label))))

(event EventTick
  (params (DeltaSeconds :type Float%20%28single-precision%29))
  (bind _camerareference (Variables|Default|GetCameraReference)
    (:then
      (Transformation|SetActorRotation (Math|Rotator|FindLookatRotation (Transformation|GetActorLocation _camerareference) (Transformation|GetActorLocation))))
    (:else)))

(fn ConstructionScript
  (if (Variables|Default|GetReducingInitative?)
    (Rendering|Components|TextRender|SetText (Variables|Default|GetTextRender) (Utilities|Text|FormatText "-{initative}" (Utilities|Text|ToText(Integer) (Math|Float|Truncate (Variables|Default|GetValue)))))
    (Rendering|Components|TextRender|SetTextRenderColor (Variables|Default|GetTextRender) (Math|Color|MakeColor 0 255 255 255))
    (Variables|/Script/Engine.MovementComponent|SetVelocity (Variables|Default|GetProjectileMovement) (Math|Vector|MakeVector 0.0 0.0 2.0))
    (elif true
      (Rendering|Components|TextRender|SetText (Variables|Default|GetTextRender) (Utilities|Text|FormatText "+{healing amount}" (Utilities|Text|ToText(Integer) (Math|Float|Truncate (Variables|Default|GetValue)))))
      (Variables|/Script/Engine.MovementComponent|SetVelocity (Variables|Default|GetProjectileMovement) (Math|Vector|MakeVector 0.0 0.0 2.0))
      (if (Variables|Default|GetRestoringMP?)
        (Rendering|Components|TextRender|SetTextRenderColor (Variables|Default|GetTextRender) (Math|Color|MakeColor 255 0 0 255))
        (else
          (Rendering|Components|TextRender|SetTextRenderColor (Variables|Default|GetTextRender) (Math|Color|MakeColor 0 255 0 255))))
      (else
        (Rendering|Components|TextRender|SetText (Variables|Default|GetTextRender) (Utilities|Text|FormatText "-{damage}" (Utilities|Text|ToText(Integer) (Math|Float|Truncate (Variables|Default|GetValue)))))
        (Variables|/Script/Engine.MovementComponent|SetVelocity (Variables|Default|GetProjectileMovement) (Math|Vector|MakeVector (Math|Random|RandomFloatinRange -0.1 0.1) (Math|Random|RandomFloatinRange -0.1 0.1) 1.0))
        (if (Variables|Default|GetCritical?)
          (Rendering|Components|TextRender|SetTextRenderColor (Variables|Default|GetTextRender) (Math|Color|MakeColor 0 0 255 255))
          (Transformation|SetWorldScale3D (Variables|Default|GetTextRender) "1.500000,1.500000,1.500000"))))))
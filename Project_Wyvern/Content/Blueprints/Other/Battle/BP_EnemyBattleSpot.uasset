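; BP_EnemyBattleSpot is an actor that marks an enemy slot in a battle formation.
; Its construction script sets a text component to a label built from the Formation line (Frontline, Middleline or Backline) and the SlotIndex.
; It has no active runtime logic, as its event graph holds only disabled default events.
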(event EventBeginPlay)

(event Collision|EventActorBeginOverlap
  (params (OtherActor :type Actor%20Object%20Reference)))

(event EventTick
  (params (DeltaSeconds :type Float%20%28single-precision%29)))

(fn ConstructionScript
  (switch Utilities|FlowControl|Switch|SwitchonE_FormationsTypes (Variables|Default|GetFormation)
    (:NewEnumerator0
      (Rendering|Components|TextRender|SetText (Variables|Default|GetText) (Utilities|Text|FormatText "Enemy 
Frontline {Index}" (Variables|Default|GetSlotIndex))))
    (:NewEnumerator1
      (Rendering|Components|TextRender|SetText (Variables|Default|GetText) (Utilities|Text|FormatText "Enemy 
Middleline {Index}" (Variables|Default|GetSlotIndex))))
    (:NewEnumerator2
      (Rendering|Components|TextRender|SetText (Variables|Default|GetText) (Utilities|Text|FormatText "Enemy 
Backline {Index}" (Variables|Default|GetSlotIndex))))))
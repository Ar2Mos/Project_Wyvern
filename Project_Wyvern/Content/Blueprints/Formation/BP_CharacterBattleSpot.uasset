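; BP_CharacterBattleSpot is a formation marker for a character's battle slot, with frontline, middleline and backline labels.
; Its construction script formats SlotIndex into the three text components, so each label shows its row and slot number.
; The event graph holds only empty, disabled default events, so the Blueprint adds no runtime logic.
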(event EventBeginPlay)

(event Collision|EventActorBeginOverlap
  (params (OtherActor :type Actor%20Object%20Reference)))

(event EventTick
  (params (DeltaSeconds :type Float%20%28single-precision%29)))

(fn ConstructionScript
  (Rendering|Components|TextRender|SetText (Variables|Default|GetFrontlineText) (Utilities|Text|FormatText "Character 
Frontline {Index}" (Variables|Default|GetSlotIndex)))
  (Rendering|Components|TextRender|SetText (Variables|Default|GetMiddlelineText) (Utilities|Text|FormatText "Character 
Middleline {Index}" (Variables|Default|GetSlotIndex)))
  (Rendering|Components|TextRender|SetText (Variables|Default|GetBacklineText) (Utilities|Text|FormatText "Character 
Backline {Index}" (Variables|Default|GetSlotIndex))))
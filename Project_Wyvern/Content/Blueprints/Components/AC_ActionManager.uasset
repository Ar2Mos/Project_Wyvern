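; Turn-based battle component that runs the current character's chosen action: attack, magic, defend or flee.
; SelectAction stores the choice, opening targeting for attacks and the Fire Ball and Cold Bolt spells, while defend and flee resolve immediately.
; ActivateActionEffect applies attack (Berserk-boosted), defend or flee, with no magic case, via sibling battle and targeting managers.
; GetActionCost derives HP/SP costs from DT_Actions and action levels stored in the game instance.
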(event EventBeginPlay
  (bind _asbp_gi_custom (Utilities|Casting|CastToBP_GI_Custom (Game|GetGameInstance) :!label _label)
    (:then
      (Variables|Default|SetGameInstanceRef _asbp_gi_custom))
    (:CastFailed
      (Utilities|FlowControl|Delay 0.2)
      (goto _label))))

(event Custom|SelectAction
  (params (ActionType :type E_ActionType%20Enum :default "NewEnumerator0") (SecondaryActionName :type Name))
  (bind _owningcharacter (Utilities|GetCurrentCharacter))
  (bind _ac_character_battlestats (Variables|/Game/Blueprints/Essential/BP_Character_Battle_Base.BP_Character_Battle_Base_C|GetAC_Character_BattleStats _owningcharacter))
  (Variables|/Game/Blueprints/Components/AC_Character_BattleStats.AC_Character_BattleStats_C|SetSelectedActionType _ac_character_battlestats ActionType)
  (Variables|/Game/Blueprints/Components/AC_Character_BattleStats.AC_Character_BattleStats_C|SetSelectedSecondaryActionName _ac_character_battlestats SecondaryActionName)
  (switch Utilities|FlowControl|Switch|SwitchonE_ActionType ActionType
    (:NewEnumerator1
      (Selection|SelectedAttack))
    (:NewEnumerator2
      (|MagicSelection))
    (:NewEnumerator3
      (Selection|SelectedDefence))
    (:NewEnumerator5
      (Selection|SelectedFlee))))

(event Custom|ActivateActionEffect
  (bind _owningcharacter (Utilities|GetCurrentCharacter))
  (Development|PrintString (Utilities|GetDisplayName _owningcharacter))
  (switch Utilities|FlowControl|Switch|SwitchonE_ActionType (Variables|/Game/Blueprints/Components/AC_Character_BattleStats.AC_Character_BattleStats_C|GetSelectedActionType (Variables|/Game/Blueprints/Essential/BP_Character_Battle_Base.BP_Character_Battle_Base_C|GetAC_Character_BattleStats _owningcharacter))
    (:NewEnumerator1
      (Activation|ActiveAttack))
    (:NewEnumerator3
      (Activation|ActiveDefend))
    (:NewEnumerator5
      (Activation|ActiveFlee))))

(fn SelectedAttack
  (Default|ShowBattleToolTip (Utilities|GetBattleManager) "Select target")
  (Default|EnableTarget (Utilities|GetTargetingManager) false "NewEnumerator1"))

(fn SelectedDefence
  (Default|DisableTargetingandInput (Utilities|GetBattleManager))
  (Activation|ActiveDefend))

(fn ActiveDefend
  (bind _battlemanager (Utilities|GetBattleManager))
  (Default|ShowBattleToolTip (Utilities|GetBattleManager) (Utilities|Text|FormatText "{char name} defends!!" (.Character%20Display%20Name (Utilities|GetCurrentCharacterName))))
  (Variables|/Game/Blueprints/Components/AC_Character_BattleStats.AC_Character_BattleStats_C|SetDefending (Variables|/Game/Blueprints/Essential/BP_Character_Battle_Base.BP_Character_Battle_Base_C|GetAC_Character_BattleStats (Utilities|GetCurrentCharacter)) true)
  (Default|EndCharacterTurn _battlemanager 1e+03)
  (Default|ResumeBattle _battlemanager))

(fn SelectedMagicFireball
  (Default|ShowBattleToolTip (Utilities|GetBattleManager) "Select target")
  (Default|EnableTarget (Utilities|GetTargetingManager) false "NewEnumerator1"))

(fn SelectedMagicColdBolt
  (Default|ShowBattleToolTip (Utilities|GetBattleManager) "Select target")
  (Default|EnableTarget (Utilities|GetTargetingManager) false "NewEnumerator1"))

(fn SelectedFlee
  (Default|DisableTargetingandInput (Utilities|GetBattleManager))
  (Activation|ActiveFlee))

(fn ActiveFlee
  (Default|GoBacktoWorldMap (Utilities|GetBattleManager)))

(fn GetActionCost
  (params (ActionName :type Name))
  (bind _charactercodedname (Utilities|GetCurrentCharacterName))
  (bind _gameinstanceref (Variables|Default|GetGameInstanceRef))
  (bind _characterscollection (Variables|/Game/Blueprints/Essential/BP_GI_Custom.BP_GI_Custom_C|GetCharactersCollection _gameinstanceref))
  (bind _value (Utilities|Map|Find _characterscollection _charactercodedname))
  (bind _chacracteractions (Utilities|Struct|BreakS_CharacterStatus _value))
  (bind _value_2 (Utilities|Map|Find _chacracteractions ActionName))
  (bind _returnvalue (Utilities|GetDataTableRow "/Game/Blueprints/DataBases/DT_Actions.DT_Actions" ActionName)
    (:then
      (return (+ (.BaseCostHP (Utilities|Struct|BreakS_Action _returnvalue)) (* _value_2 (.PerLevelCostHP (Utilities|Struct|BreakS_Action _returnvalue)))) (+ (.BaseCostSP (Utilities|Struct|BreakS_Action _returnvalue)) (* _value_2 (.PerLevelCostSP (Utilities|Struct|BreakS_Action _returnvalue))))))))

(fn ActiveAttack
  (bind _owningcharacter (Utilities|GetCurrentCharacter))
  (bind _owningcharacter_2 (Utilities|GetCurrentCharacter))
  (bind _ac_character_battlestats (Variables|/Game/Blueprints/Essential/BP_Character_Battle_Base.BP_Character_Battle_Base_C|GetAC_Character_BattleStats _owningcharacter))
  (bind _ac_character_battlestats_2 (Variables|/Game/Blueprints/Essential/BP_Character_Battle_Base.BP_Character_Battle_Base_C|GetAC_Character_BattleStats _owningcharacter_2))
  (bind _character_stats (Variables|/Game/Blueprints/Components/AC_Character_BattleStats.AC_Character_BattleStats_C|GetCharacter%20Stats _ac_character_battlestats_2))
  (bind _berserk_ (Variables|/Game/Blueprints/Components/AC_Character_BattleStats.AC_Character_BattleStats_C|GetBerserk? _ac_character_battlestats))
  (for _array_element (Variables|/Game/Blueprints/Components/AC_Character_BattleStats.AC_Character_BattleStats_C|GetTargetedCharacter _ac_character_battlestats)
    (Development|PrintString (Utilities|GetDisplayName (Variables|/Game/Blueprints/Essential/BP_Character_Battle_Base.BP_Character_Battle_Base_C|GetAC_Character_BattleStats _array_element)))
    (Default|ReceiveDamage (Variables|/Game/Blueprints/Essential/BP_Character_Battle_Base.BP_Character_Battle_Base_C|GetAC_Character_BattleStats _array_element) (* (.Value (Utilities|Map|Find _character_stats "NewEnumerator9")) (Math|Float|SelectFloat 1.3 1.0 _berserk_)) (+ (.Value (Utilities|Map|Find _character_stats "NewEnumerator8")) (Math|Float|SelectFloat 1e+01 1.0 _berserk_)) (.Value (Utilities|Map|Find _character_stats "NewEnumerator10")))))
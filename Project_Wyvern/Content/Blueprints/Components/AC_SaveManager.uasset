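; Actor component for a jRPG that manages save bookkeeping, new-game setup and world-map spawn data, keeping live state in BP_GI_Custom.
; A SavesContainer slot indexes save names, while SaveGametoFile fills a BP_Gamesave with map, time and area without writing it.
; StartNewGame resets the game instance, seeds characters and items from data tables, then changes map.
; Tick accumulates play time and optionally refreshes the world HUD.
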(event EventBeginPlay
  (bind _asbp_gi_custom (Utilities|Casting|CastToBP_GI_Custom (Game|GetGameInstance) :!label _label)
    (:then
      (Variables|Default|SetGameInstanceReference _asbp_gi_custom))
    (:CastFailed
      (Utilities|FlowControl|Delay 0.2)
      (goto _label))))

(event EventTick
  (params (DeltaSeconds :type Float%20%28single-precision%29))
  (bind _gameinstancereference (Variables|Default|GetGameInstanceReference)
    (:then
      (Variables|/Game/Blueprints/Essential/BP_GI_Custom.BP_GI_Custom_C|SetTimePlayed _gameinstancereference (+ (Class|ActorComponent|GetComponentTickInterval) (Variables|/Game/Blueprints/Essential/BP_GI_Custom.BP_GI_Custom_C|GetTimePlayed _gameinstancereference)))
      (if (Variables|Default|GetAutoRefreshTimePlayed?)
        (TimePlayed|RefreshTimePlayed)))
    (:else)))

(fn LoadSavesContainer
  (bind _returnvalue (SaveGame|DoesSaveGameExist "AvailableSaves"))
  (if _returnvalue
    (bind _returnvalue_2 (SaveGame|LoadGamefromSlot "SavesContainer"))
    (bind _asbp_saves_container (Utilities|Casting|CastToBP_SavesContainer _returnvalue_2))
    (LocalVariables|SetAvailableSaves (Variables|/Game/Blueprints/SaveObj/BP_SavesContainer.BP_SavesContainer_C|GetAllSaves _asbp_saves_container))
    (else
      (bind _returnvalue_3 (SaveGame|CreateSaveGameObject "/Game/Blueprints/SaveObj/BP_SavesContainer.BP_SavesContainer_C"))
      (SaveGame|SaveGametoSlot _returnvalue_3 "SavesContainer"))))

(fn AddNewSavetoSavesContainer
  (params (SaveName :type String))
  (bind _returnvalue (SaveGame|DoesSaveGameExist "SavesContainer"))
  (if _returnvalue
    (Utilities|Array|Add (LocalVariables|GetAvailableSaves) SaveName)
    (bind _returnvalue_2 (SaveGame|LoadGamefromSlot "SavesContainer"))
    (bind _asbp_saves_container (Utilities|Casting|CastToBP_SavesContainer _returnvalue_2))
    (bind _output_get (LocalVariables|SetAllSavesLocal (Variables|/Game/Blueprints/SaveObj/BP_SavesContainer.BP_SavesContainer_C|GetAllSaves _asbp_saves_container)))
    (Utilities|Array|Add _output_get SaveName)
    (Variables|/Game/Blueprints/SaveObj/BP_SavesContainer.BP_SavesContainer_C|SetAllSaves _asbp_saves_container (LocalVariables|GetAllSavesLocal))
    (SaveGame|SaveGametoSlot _asbp_saves_container "SavesContainer")))

(fn RemoveSavefromSavesContainer
  (params (SaveName :type String))
  (bind _returnvalue (SaveGame|DoesSaveGameExist "SavesContainer"))
  (if _returnvalue
    (Utilities|Array|RemoveItem (LocalVariables|GetAvailableSaves) SaveName)
    (bind _returnvalue_2 (SaveGame|LoadGamefromSlot "SavesContainer"))
    (bind _asbp_saves_container (Utilities|Casting|CastToBP_SavesContainer _returnvalue_2))
    (bind _output_get (LocalVariables|SetAllSavesLocal (Variables|/Game/Blueprints/SaveObj/BP_SavesContainer.BP_SavesContainer_C|GetAllSaves _asbp_saves_container)))
    (Utilities|Array|RemoveItem _output_get SaveName)
    (Variables|/Game/Blueprints/SaveObj/BP_SavesContainer.BP_SavesContainer_C|SetAllSaves _asbp_saves_container (LocalVariables|GetAllSavesLocal))
    (SaveGame|SaveGametoSlot _asbp_saves_container "SavesContainer")))

(fn GetonLoadMapTransform
  (bind _gameinstancereference (Variables|Default|GetGameInstanceReference))
  (bind _worldmapspawnpointname (Variables|/Game/Blueprints/Essential/BP_GI_Custom.BP_GI_Custom_C|GetWorldMapSpawnPointName _gameinstancereference))
  (bind _spawnpoint (MapChanging|Functionality|GetMapSpawnPointwithName _worldmapspawnpointname))
  (if (Variables|/Game/Blueprints/Essential/BP_GI_Custom.BP_GI_Custom_C|GetSpawningAfterBattle? _gameinstancereference)
    (Variables|/Game/Blueprints/Essential/BP_GI_Custom.BP_GI_Custom_C|SetSpawningAfterBattle? (Variables|Default|GetGameInstanceReference) false)
    (return (Variables|/Game/Blueprints/Essential/BP_GI_Custom.BP_GI_Custom_C|GetWorldTransformBeforeBattle _gameinstancereference) (Variables|/Game/Blueprints/Essential/BP_GI_Custom.BP_GI_Custom_C|GetCameraWorldRotationBeforeBattle _gameinstancereference))
    (else
      (Utilities|IsValid _spawnpoint
        (:Is%20Valid
          (return (LocalVariables|GetDefaultTransform) (LocalVariables|GetDefaultCameraRotation)))
        (:Is%20Not%20Valid
          (return (Default|GetSpawnTransform _spawnpoint) (LocalVariables|GetDefaultCameraRotation)))))))

(fn GetMapSpawnPointwithName
  (params (SpawnPointName :type Name))
  (bind _outactors (Actor|GetAllActorsOfClass "/Game/Blueprints/Other/World/BP_MapSpawnPoint.BP_MapSpawnPoint_C"))
  (bind _array_element (Utilities|Array|ForEachLoopwithBreak _outactors :!label _label)
    (:LoopBody
      (if (== (Variables|/Game/Blueprints/Other/World/BP_MapSpawnPoint.BP_MapSpawnPoint_C|GetSpawnPointName _array_element) SpawnPointName)
        (LocalVariables|SetSpawnPointLocal _array_element)
        (goto _label Break)))
    (:Completed
      (return (LocalVariables|GetSpawnPointLocal)))))

(fn ChangeAreaName
  (params (NewAreaName :type Text))
  (bind _gameinstancereference (Variables|Default|GetGameInstanceReference)
    (:then
      (Variables|/Game/Blueprints/Essential/BP_GI_Custom.BP_GI_Custom_C|SetAreaName _gameinstancereference NewAreaName)
      (MapChanging|Widgets|RefreshAreaName))
    (:else)))

(fn RefreshAreaName
  (bind _foundwidgets (Widget|GetAllWidgetsOfClass "/Game/widgets/Widgets/WorldInterface/WBP_jRPG_WorldInterface.WBP_jRPG_WorldInterface_C" false))
  (Utilities|IsValid (Utilities|Array|Get(acopy) _foundwidgets)
    (:Is%20Valid
      (Rendering|Components|TextRender|SetText (Variables|/Game/widgets/Widgets/WorldInterface/WBP_jRPG_WorldInterface.WBP_jRPG_WorldInterface_C|GetTextBlock_AreaName (Utilities|Array|Get(acopy) _foundwidgets)) (Variables|/Game/Blueprints/Essential/BP_GI_Custom.BP_GI_Custom_C|GetAreaName (Variables|Default|GetGameInstanceReference))))))

(fn RefreshTimePlayed
  (bind _foundwidgets (Widget|GetAllWidgetsOfClass "/Game/widgets/Widgets/WorldInterface/WBP_jRPG_WorldInterface.WBP_jRPG_WorldInterface_C" true))
  (Utilities|IsValid (Utilities|Array|Get(acopy) _foundwidgets)
    (:Is%20Valid
      (Rendering|Components|TextRender|SetText (Variables|/Game/widgets/Widgets/WorldInterface/WBP_jRPG_WorldInterface.WBP_jRPG_WorldInterface_C|GetTextBlock_TimePlayed (Utilities|Array|Get(acopy) _foundwidgets)) (Utilities|GetTimeasText (Variables|/Game/Blueprints/Essential/BP_GI_Custom.BP_GI_Custom_C|GetTimePlayed (Variables|Default|GetGameInstanceReference)))))))

(fn SaveGametoFile
  (params (SaveOverview :type String))
  (bind _output_get (LocalVariables|SetCreateNewSave?Local (Utilities|Enum|Equal(Enum) SaveOverview "")))
  (if _output_get
    (LocalVariables|SetSaveNameLocal (Utilities|GetCurrentTimeasString))
    (else
      (LocalVariables|SetSaveNameLocal SaveOverview)))
  (bind _returnvalue (SaveGame|CreateSaveGameObject "/Game/Blueprints/SaveObj/BP_Gamesave.BP_Gamesave_C"))
  (LocalVariables|SetSaveReferenceLocal _returnvalue)
  (Utilities|FlowControl|Sequence
    (:then_0
      (bind _returnvalue_2 (Game|GetCurrentLevelName true))
      (Variables|/Game/Blueprints/SaveObj/BP_Gamesave.BP_Gamesave_C|SetMapToLoad (LocalVariables|GetSaveReferenceLocal) (Utilities|String|StringToName _returnvalue_2))
      (Variables|/Game/Blueprints/SaveObj/BP_Gamesave.BP_Gamesave_C|SetTimePlayed (LocalVariables|GetSaveReferenceLocal) (Variables|/Game/Blueprints/Essential/BP_GI_Custom.BP_GI_Custom_C|GetTimePlayed (Variables|Default|GetGameInstanceReference)))
      (Variables|/Game/Blueprints/SaveObj/BP_Gamesave.BP_Gamesave_C|SetAreaName (LocalVariables|GetSaveReferenceLocal) (Variables|/Game/Blueprints/Essential/BP_GI_Custom.BP_GI_Custom_C|GetAreaName (Variables|Default|GetGameInstanceReference))))))

(fn StartNewGame
  (bind _returnvalue (Components|GetOwner))
  (bind _gameinstancereference (Variables|Default|GetGameInstanceReference))
  (bind _defaultitemslocal (LocalVariables|GetDefaultItemsLocal))
  (bind _gameinstancereference_2 (Variables|Default|GetGameInstanceReference))
  (bind _returnvalue_2 (Actor|GetComponentbyClass _returnvalue "/Game/Blueprints/Components/AC_CharacterManager.AC_CharacterManager_C"))
  (Utilities|Map|Clear (Variables|/Game/Blueprints/Essential/BP_GI_Custom.BP_GI_Custom_C|GetCharactersCollection _gameinstancereference_2))
  (Utilities|Array|Clear (Variables|/Game/Blueprints/Essential/BP_GI_Custom.BP_GI_Custom_C|GetCurrentParty _gameinstancereference_2))
  (Utilities|Array|Clear (Variables|/Game/Blueprints/Essential/BP_GI_Custom.BP_GI_Custom_C|GetInventory (Variables|Default|GetGameInstanceReference)))
  (Variables|/Game/Blueprints/Essential/BP_GI_Custom.BP_GI_Custom_C|SetTimePlayed (Variables|Default|GetGameInstanceReference) 0.0)
  (Utilities|FlowControl|Sequence
    (:then_0
      (Utilities|IsValid _returnvalue_2
        (:Is%20Valid
          (for _array_element (LocalVariables|GetDefaultCharactersLocal)
            (bind _returnvalue_3 (Utilities|GetDataTableRow "/Game/Blueprints/DataBases/DT_Character.DT_Character" _array_element)
              (:then
                (Default|AddNewCharactertoCollection _returnvalue_2 _returnvalue_3)))))))
    (:then_1
      (Variables|/Game/Blueprints/Essential/BP_GI_Custom.BP_GI_Custom_C|SetCurrentParty (Variables|Default|GetGameInstanceReference) (LocalVariables|GetDefaultPartyLocal)))
    (:then_2
      (Variables|/Game/Blueprints/Essential/BP_GI_Custom.BP_GI_Custom_C|SetZeny (Variables|Default|GetGameInstanceReference) (LocalVariables|GetDefaultZenyAmountLocal))
      (bind _keys (Utilities|Map|Keys _defaultitemslocal))
      (for _array_element_2 _keys
        (bind _returnvalue_4 (Utilities|GetDataTableRow "/Game/Blueprints/DataBases/DT_Items.DT_Items" _array_element_2)
          (:then
            (Utilities|Array|Add (Variables|/Game/Blueprints/Essential/BP_GI_Custom.BP_GI_Custom_C|GetInventory (Variables|Default|GetGameInstanceReference)) (Utilities|Struct|MakeS_Items_Dynamic (.Value (Utilities|Map|Find _defaultitemslocal _array_element_2)) _returnvalue_4))))))
    (:then_3
      (Variables|/Game/Blueprints/Essential/BP_GI_Custom.BP_GI_Custom_C|SetAreaName (Variables|Default|GetGameInstanceReference) (LocalVariables|GetDefaultAreaName)))
    (:then_4
      (Variables|/Game/Blueprints/Essential/BP_GI_Custom.BP_GI_Custom_C|SetInteractedObjects _gameinstancereference (Utilities|Map|MakeMap))
      (Variables|/Game/Blueprints/Essential/BP_GI_Custom.BP_GI_Custom_C|SetBattledEnemies _gameinstancereference (Utilities|Map|MakeMap)))
    (:then_5
      (CallFunction|ChangeMap "Map_World1" "SpawnA"))))
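; Actor component that manages target selection in turn-based battles, from self or single characters to formation rows and whole sides.
; EnableTarget stores the targeting type and self-target flag, then switches the owner's AC_CameraManager to an ally or enemy camera path.
; ShowTarget reveals pointers on valid characters from the BattleManager's lists and records them in TargetedCharacters; HideTarget clears them.
; CancelTargeting restores the general ally camera path; BeginPlay retries caching the game instance.
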(event EventBeginPlay
  (bind _asbp_gi_custom (Utilities|Casting|CastToBP_GI_Custom (Game|GetGameInstance) :!label _label)
    (:then
      (Variables|Default|SetGame%20Instance%20Reference _asbp_gi_custom))
    (:CastFailed
      (Utilities|FlowControl|Delay 0.1)
      (goto _label))))

(fn EnableTarget
  (params (CanTargetSelf? :type Boolean) (TargetingType :type E_TargetType%20Enum :default "NewEnumerator0"))
  (Variables|Default|SetCanTargetSelf? CanTargetSelf?)
  (Variables|Default|SetSelectedTargetType TargetingType)
  (Variables|Default|SetTargetEnabled? true)
  (switch Utilities|FlowControl|Switch|SwitchonE_TargetType (Variables|Default|GetSelectedTargetType)
    (:NewEnumerator0
      (Default|SetNewDynamicPath (Actor|GetComponentbyClass (Components|GetOwner) "/Game/Blueprints/Components/AC_CameraManager.AC_CameraManager_C") "Ally_Targeting" true true false "0, 0, 0" :!label _label))
    (:NewEnumerator1
      (Default|SetNewDynamicPath (Actor|GetComponentbyClass (Components|GetOwner) "/Game/Blueprints/Components/AC_CameraManager.AC_CameraManager_C") "Enemy_Target" true true false "0, 0, 0" :!label _label_2))
    (:NewEnumerator2
      (goto _label))
    (:NewEnumerator3
      (goto _label_2))
    (:NewEnumerator4
      (goto _label))
    (:NewEnumerator5
      (goto _label_2))
    (:NewEnumerator6
      (goto _label))))

(fn DisableTarget
  (Variables|Default|SetTargetEnabled? false))

(fn ShowTarget
  (params (IndicatedCharacter :type BP%20Character%20Battle%20Base%20Object%20Reference))
  (LocalVariables|SetIndicatedCharacterLocal IndicatedCharacter)
  (switch Utilities|FlowControl|Switch|SwitchonE_TargetType (Variables|Default|GetSelectedTargetType)
    (:NewEnumerator0
      (if (== (Variables|/Game/Blueprints/Components/AC_BattleManager.AC_BattleManager_C|GetCurrentCharacter (Variables|/Game/Blueprints/Essential/BP_Character_Battle_Base.BP_Character_Battle_Base_C|GetBattleManagerReference (LocalVariables|GetIndicatedCharacterLocal))) (LocalVariables|GetIndicatedCharacterLocal))
        (Development|SetHiddeninGame (Variables|/Game/Blueprints/Essential/BP_Character_Battle_Base.BP_Character_Battle_Base_C|GetTargetPointer (LocalVariables|GetIndicatedCharacterLocal)) false false)
        (Utilities|Array|Add (Variables|Default|GetTargetedCharacters) (LocalVariables|GetIndicatedCharacterLocal))))
    (:NewEnumerator1
      (if (Variables|/Game/Blueprints/Essential/BP_Character_Battle_Base.BP_Character_Battle_Base_C|GetEnemy? (LocalVariables|GetIndicatedCharacterLocal))
        (Development|SetHiddeninGame (Variables|/Game/Blueprints/Essential/BP_Character_Battle_Base.BP_Character_Battle_Base_C|GetTargetPointer (LocalVariables|GetIndicatedCharacterLocal)) false false)
        (Utilities|Array|Add (Variables|Default|GetTargetedCharacters) (LocalVariables|GetIndicatedCharacterLocal))))
    (:NewEnumerator2
      (if (not (Variables|/Game/Blueprints/Essential/BP_Character_Battle_Base.BP_Character_Battle_Base_C|GetEnemy? (LocalVariables|GetIndicatedCharacterLocal)))
        (if (Variables|Default|GetCanTargetSelf?)
          (Development|SetHiddeninGame (Variables|/Game/Blueprints/Essential/BP_Character_Battle_Base.BP_Character_Battle_Base_C|GetTargetPointer (LocalVariables|GetIndicatedCharacterLocal)) false false :!label _label)
          (Utilities|Array|Add (Variables|Default|GetTargetedCharacters) (LocalVariables|GetIndicatedCharacterLocal))
          (elif (!= (Variables|/Game/Blueprints/Components/AC_BattleManager.AC_BattleManager_C|GetCurrentCharacter (Variables|/Game/Blueprints/Essential/BP_Character_Battle_Base.BP_Character_Battle_Base_C|GetBattleManagerReference (LocalVariables|GetIndicatedCharacterLocal))) (LocalVariables|GetIndicatedCharacterLocal))
            (goto _label)))))
    (:NewEnumerator3
      (if (Variables|/Game/Blueprints/Essential/BP_Character_Battle_Base.BP_Character_Battle_Base_C|GetEnemy? (LocalVariables|GetIndicatedCharacterLocal))
        (for _array_element (Variables|/Game/Blueprints/Components/AC_BattleManager.AC_BattleManager_C|GetEnemies (Variables|/Game/Blueprints/Essential/BP_Character_Battle_Base.BP_Character_Battle_Base_C|GetBattleManagerReference (LocalVariables|GetIndicatedCharacterLocal)))
          (if (Utilities|Enum|Equal(Enum) (Variables|/Game/Blueprints/Essential/BP_Character_Battle_Base.BP_Character_Battle_Base_C|GetFormationType _array_element) (Variables|/Game/Blueprints/Essential/BP_Character_Battle_Base.BP_Character_Battle_Base_C|GetFormationType (LocalVariables|GetIndicatedCharacterLocal)))
            (Development|SetHiddeninGame (Variables|/Game/Blueprints/Essential/BP_Character_Battle_Base.BP_Character_Battle_Base_C|GetTargetPointer _array_element) false false)
            (Utilities|Array|Add (Variables|Default|GetTargetedCharacters) _array_element)))))
    (:NewEnumerator4
      (if (not (Variables|/Game/Blueprints/Essential/BP_Character_Battle_Base.BP_Character_Battle_Base_C|GetEnemy? (LocalVariables|GetIndicatedCharacterLocal)))
        (for _array_element_2 (Variables|/Game/Blueprints/Components/AC_BattleManager.AC_BattleManager_C|GetPlayerCharacters (Variables|/Game/Blueprints/Essential/BP_Character_Battle_Base.BP_Character_Battle_Base_C|GetBattleManagerReference (LocalVariables|GetIndicatedCharacterLocal)))
          (if (Utilities|Enum|Equal(Enum) (Variables|/Game/Blueprints/Essential/BP_Character_Battle_Base.BP_Character_Battle_Base_C|GetFormationType _array_element_2) (Variables|/Game/Blueprints/Essential/BP_Character_Battle_Base.BP_Character_Battle_Base_C|GetFormationType (LocalVariables|GetIndicatedCharacterLocal)))
            (if (Variables|Default|GetCanTargetSelf?)
              (Development|SetHiddeninGame (Variables|/Game/Blueprints/Essential/BP_Character_Battle_Base.BP_Character_Battle_Base_C|GetTargetPointer _array_element_2) false false :!label _label_2)
              (Utilities|Array|Add (Variables|Default|GetTargetedCharacters) _array_element_2)
              (elif (!= _array_element_2 (Variables|/Game/Blueprints/Components/AC_BattleManager.AC_BattleManager_C|GetCurrentCharacter (Variables|/Game/Blueprints/Essential/BP_Character_Battle_Base.BP_Character_Battle_Base_C|GetBattleManagerReference (LocalVariables|GetIndicatedCharacterLocal))))
                (goto _label_2)))))))
    (:NewEnumerator5
      (if (Variables|/Game/Blueprints/Essential/BP_Character_Battle_Base.BP_Character_Battle_Base_C|GetEnemy? (LocalVariables|GetIndicatedCharacterLocal))
        (for _array_element_3 (Variables|/Game/Blueprints/Components/AC_BattleManager.AC_BattleManager_C|GetEnemies (Variables|/Game/Blueprints/Essential/BP_Character_Battle_Base.BP_Character_Battle_Base_C|GetBattleManagerReference (LocalVariables|GetIndicatedCharacterLocal)))
          (Development|SetHiddeninGame (Variables|/Game/Blueprints/Essential/BP_Character_Battle_Base.BP_Character_Battle_Base_C|GetTargetPointer _array_element_3) false false)
          (Utilities|Array|Add (Variables|Default|GetTargetedCharacters) _array_element_3))))
    (:NewEnumerator6
      (if (not (Variables|/Game/Blueprints/Essential/BP_Character_Battle_Base.BP_Character_Battle_Base_C|GetEnemy? (LocalVariables|GetIndicatedCharacterLocal)))
        (for _array_element_4 (Variables|/Game/Blueprints/Components/AC_BattleManager.AC_BattleManager_C|GetPlayerCharacters (Variables|/Game/Blueprints/Essential/BP_Character_Battle_Base.BP_Character_Battle_Base_C|GetBattleManagerReference (LocalVariables|GetIndicatedCharacterLocal)))
          (if (Variables|Default|GetCanTargetSelf?)
            (Development|SetHiddeninGame (Variables|/Game/Blueprints/Essential/BP_Character_Battle_Base.BP_Character_Battle_Base_C|GetTargetPointer _array_element_4) false false :!label _label_3)
            (Utilities|Array|Add (Variables|Default|GetTargetedCharacters) _array_element_4)
            (elif (!= _array_element_4 (Variables|/Game/Blueprints/Components/AC_BattleManager.AC_BattleManager_C|GetCurrentCharacter (Variables|/Game/Blueprints/Essential/BP_Character_Battle_Base.BP_Character_Battle_Base_C|GetBattleManagerReference (LocalVariables|GetIndicatedCharacterLocal))))
              (goto _label_3))))))))

(fn HideTarget
  (for _array_element (Variables|Default|GetTargetedCharacters)
    (Development|SetHiddeninGame (Variables|/Game/Blueprints/Essential/BP_Character_Battle_Base.BP_Character_Battle_Base_C|GetTargetPointer _array_element) true false))
  (Utilities|Array|Clear (Variables|Default|GetTargetedCharacters)))

(fn CancelTargeting
  (if (Variables|Default|GetTargetEnabled?)
    (Variables|Default|SetTargetEnabled? false)
    (Default|SetNewDynamicPath (Actor|GetComponentbyClass (Components|GetOwner) "/Game/Blueprints/Components/AC_CameraManager.AC_CameraManager_C") "Ally_Genaral" true true false "0, 0, 0")))
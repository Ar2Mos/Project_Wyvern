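; Actor component that manages turn-based jRPG battles and travel between world and battle maps.
; BP_GI_Custom carries encounter, party and world transforms across level loads, receiving HP/SP back afterward.
; Party and DataTable enemies spawn at slot actors; a delayed recursive loop adds initiative until someone reaches the threshold, checking players first.
; AI characters act automatically; player turns highlight UI slots, with chosen actions forwarded to AC_ActionManager.
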(event EventBeginPlay
  (bind _asbp_gi_custom (Utilities|Casting|CastToBP_GI_Custom (Game|GetGameInstance) :!label _label)
    (:then
      (Variables|Default|SetGame%20Instance%20Reference _asbp_gi_custom))
    (:CastFailed
      (Utilities|FlowControl|Delay 0.1)
      (goto _label))))

(event Custom|ResumeBattle
  (CallFunction|AddInitativetoAllChars))

(event Custom|AddInitativeToAllChars
  (Utilities|FlowControl|Delay 0.2)
  (if (Math|Boolean|NORBoolean (== (Utilities|Array|Length (Variables|BattleinProgress|GetPlayerCharacters)) 0) (== (Utilities|Array|Length (Variables|BattleinProgress|GetEnemies)) 0))
    (bind (_success_ _character) (BattleinProgress|TurnStart|GetCharacterwithMaxInitiative))
    (if _success_
      (BattleinProgress|TurnStart|StartCharacterTurn _character)
      (else
        (for _array_element (Variables|BattleinProgress|GetPlayerCharacters)
          (Default|AddInitiative (Variables|/Game/Blueprints/Essential/BP_Character_Battle_Base.BP_Character_Battle_Base_C|GetAC_Character_BattleStats _array_element) 0.0))
        (for _array_element_2 (Variables|BattleinProgress|GetEnemies)
          (Default|AddInitiative (Variables|/Game/Blueprints/Essential/BP_Character_Battle_Base.BP_Character_Battle_Base_C|GetAC_Character_BattleStats _array_element_2) 0.0))
        (CallFunction|AddInitativetoAllChars)))))

(fn EncounterEnemies
  (params (Encounter%20Name :type Name) (Battle%20Map%20Name :type Name))
  (bind _returnvalue (Utilities|GetDataTableRow "/Game/Blueprints/DataBases/DT_Encounters.DT_Encounters" Encounter%20Name)))

(fn OpenMapBattle
  (params (Battle%20Map%20Name :type Name) (Encountered%20Enemies :type Map%20of%20Integers%20to%20Names))
  (Variables|/Game/Blueprints/Essential/BP_GI_Custom.BP_GI_Custom_C|SetEncounteredEnemies (Variables|Default|GetGame%20Instance%20Reference) Encountered%20Enemies)
  (Variables|/Game/Blueprints/Essential/BP_GI_Custom.BP_GI_Custom_C|SetWorldTransformBeforeBattle (Variables|Default|GetGame%20Instance%20Reference) (Transformation|GetActorTransform (Game|Player|GetPlayerPawn 0)))
  (Variables|/Game/Blueprints/Essential/BP_GI_Custom.BP_GI_Custom_C|SetWorldEnemyTransformBeforeBattle (Variables|Default|GetGame%20Instance%20Reference) (Pre-Battle|GetWorldEnemiesTransforms))
  (Game|OpenLevel(byName) Battle%20Map%20Name))

(fn GetWorldEnemiesTransforms
  (bind _outactors (Actor|GetAllActorsOfClass "/Game/Blueprints/Essential/BP_World_Enemy.BP_World_Enemy_C"))
  (for _array_element _outactors
    (Utilities|Map|Add (LocalVariables|GetEnemiesTransformsLocal) (Variables|/Game/Blueprints/Essential/BP_World_Enemy.BP_World_Enemy_C|GetEnemyGlobalID _array_element) (Transformation|GetActorTransform _array_element)))
  (return (LocalVariables|GetEnemiesTransformsLocal)))

(fn SpawnPlayerCharacter
  (for (_array_element _array_index) (Variables|/Game/Blueprints/Essential/BP_GI_Custom.BP_GI_Custom_C|GetCurrentParty (Variables|Default|GetGame%20Instance%20Reference))
    (bind _returnvalue (Game|SpawnActorfromClass (.CharacterActorClass (Utilities|Struct|BreakS_CharacterStatus (.Value (Utilities|Map|Find (Variables|/Game/Blueprints/Essential/BP_GI_Custom.BP_GI_Custom_C|GetCharactersCollection (Variables|Default|GetGame%20Instance%20Reference)) (.CharacterCodedName (Utilities|Struct|BreakS_PartySlot _array_element)))))) (.Battle%20Spot%20Transform (BattleBegin|GetProperBattleSpawnTransform false _array_index (.Formations (Utilities|Struct|BreakS_PartySlot _array_element)))) "Undefined" "MultiplyWithRoot" 0 self (Actor|GetComponentbyClass (Components|GetOwner) "/Game/Blueprints/Components/AC_TargetManager.AC_TargetManager_C") false false (.BattleSpotFormationType (BattleBegin|GetProperBattleSpawnTransform false _array_index (.Formations (Utilities|Struct|BreakS_PartySlot _array_element)))) 0))
    (Default|SetCharacterData (Variables|/Game/Blueprints/Essential/BP_Character_Battle_Base.BP_Character_Battle_Base_C|GetAC_Character_BattleStats _returnvalue) (.CharacterDisplayName (Utilities|Struct|BreakS_CharacterStatus (.Value (Utilities|Map|Find (Variables|/Game/Blueprints/Essential/BP_GI_Custom.BP_GI_Custom_C|GetCharactersCollection (Variables|Default|GetGame%20Instance%20Reference)) (.CharacterCodedName (Utilities|Struct|BreakS_PartySlot _array_element)))))) (.CharacterStats (Utilities|Struct|BreakS_CharacterStatus (.Value (Utilities|Map|Find (Variables|/Game/Blueprints/Essential/BP_GI_Custom.BP_GI_Custom_C|GetCharactersCollection (Variables|Default|GetGame%20Instance%20Reference)) (.CharacterCodedName (Utilities|Struct|BreakS_PartySlot _array_element)))))) (.CurrentHP (Utilities|Struct|BreakS_CharacterStatus (.Value (Utilities|Map|Find (Variables|/Game/Blueprints/Essential/BP_GI_Custom.BP_GI_Custom_C|GetCharactersCollection (Variables|Default|GetGame%20Instance%20Reference)) (.CharacterCodedName (Utilities|Struct|BreakS_PartySlot _array_element)))))) (.CurrentSP (Utilities|Struct|BreakS_CharacterStatus (.Value (Utilities|Map|Find (Variables|/Game/Blueprints/Essential/BP_GI_Custom.BP_GI_Custom_C|GetCharactersCollection (Variables|Default|GetGame%20Instance%20Reference)) (.CharacterCodedName (Utilities|Struct|BreakS_PartySlot _array_element)))))))
    (Utilities|Array|Add (Variables|BattleinProgress|GetPlayerCharacters) _returnvalue)
    (Default|CreateCharacterBattleSlot (Variables|/Game/Blueprints/Essential/BP_Character_Battle_Base.BP_Character_Battle_Base_C|GetAC_Character_BattleStats _returnvalue))
    (Variables|/Game/Blueprints/Components/AC_Character_BattleStats.AC_Character_BattleStats_C|SetBattleManagerReference (Variables|/Game/Blueprints/Essential/BP_Character_Battle_Base.BP_Character_Battle_Base_C|GetAC_Character_BattleStats _returnvalue) self)
    (if (== (Variables|/Game/Blueprints/Components/AC_Character_BattleStats.AC_Character_BattleStats_C|GetCurrent%20HP (Variables|/Game/Blueprints/Essential/BP_Character_Battle_Base.BP_Character_Battle_Base_C|GetAC_Character_BattleStats _returnvalue)) 0.0)
      (Utilities|Array|RemoveItem (Variables|BattleinProgress|GetPlayerCharacters) _returnvalue)
      (Utilities|Array|Add (Variables|BattleinProgress|GetDeadPlayerCharacters) _returnvalue)
      (Variables|/Game/Blueprints/Essential/BP_Character_Battle_Base.BP_Character_Battle_Base_C|SetDead? _returnvalue true))))

(fn GetProperBattleSpawnTransform
  (params (EnemySpot? :type Boolean) (SpotIndex :type Integer) (FormationType :type E_FormationsTypes%20Enum :default "NewEnumerator0"))
  (if EnemySpot?
    (bind _outactors (Actor|GetAllActorsOfClass "/Game/Blueprints/Formation/BP_Enemy_BattleSpot.BP_Enemy_BattleSpot_C"))
    (bind _array_element (Utilities|Array|ForEachLoopwithBreak _outactors :!label _label)
      (:LoopBody
        (if (== (Variables|/Game/Blueprints/Formation/BP_Enemy_BattleSpot.BP_Enemy_BattleSpot_C|GetSlotIndex _array_element) SpotIndex)
          (LocalVariables|SetBattleSpotTransformLocal (Math|Transform|MakeTransform (Transformation|GetActorLocation _array_element) (.rotation (Transformation|GetWorldTransform (Variables|/Game/Blueprints/Formation/BP_Enemy_BattleSpot.BP_Enemy_BattleSpot_C|GetArrow _array_element))) (.scale (Transformation|GetWorldTransform (Variables|/Game/Blueprints/Formation/BP_Enemy_BattleSpot.BP_Enemy_BattleSpot_C|GetArrow _array_element)))))
          (goto _label Break)))
      (:Completed
        (return (LocalVariables|GetBattleSpotTransformLocal) (select (< SpotIndex 4) "NewEnumerator2" "NewEnumerator0"))))
    (else
      (bind _outactors_2 (Actor|GetAllActorsOfClass "/Game/Blueprints/Formation/BP_CharacterBattleSpot.BP_CharacterBattleSpot_C"))
      (bind _array_element_2 (Utilities|Array|ForEachLoopwithBreak _outactors_2 :!label _label_2)
        (:LoopBody
          (if (== (Variables|/Game/Blueprints/Formation/BP_CharacterBattleSpot.BP_CharacterBattleSpot_C|GetSlotIndex _array_element_2) SpotIndex)
            (LocalVariables|SetBattleSpotTransformLocal (Math|Transform|MakeTransform (Math|Vector|MakeVector (.X (Math|Vector|BreakVector (.location (Utilities|Select :Index FormationType :NewEnumerator0 (Transformation|GetWorldTransform (Variables|/Game/Blueprints/Formation/BP_CharacterBattleSpot.BP_CharacterBattleSpot_C|GetFrontlineArrow _array_element_2)) :NewEnumerator1 (Transformation|GetWorldTransform (Variables|/Game/Blueprints/Formation/BP_CharacterBattleSpot.BP_CharacterBattleSpot_C|GetMiddlelineArrow _array_element_2)) :NewEnumerator2 (Transformation|GetWorldTransform (Variables|/Game/Blueprints/Formation/BP_CharacterBattleSpot.BP_CharacterBattleSpot_C|GetBacklineArrow _array_element_2)))))) (.Y (Math|Vector|BreakVector (.location (Utilities|Select :Index FormationType :NewEnumerator0 (Transformation|GetWorldTransform (Variables|/Game/Blueprints/Formation/BP_CharacterBattleSpot.BP_CharacterBattleSpot_C|GetFrontlineArrow _array_element_2)) :NewEnumerator1 (Transformation|GetWorldTransform (Variables|/Game/Blueprints/Formation/BP_CharacterBattleSpot.BP_CharacterBattleSpot_C|GetMiddlelineArrow _array_element_2)) :NewEnumerator2 (Transformation|GetWorldTransform (Variables|/Game/Blueprints/Formation/BP_CharacterBattleSpot.BP_CharacterBattleSpot_C|GetBacklineArrow _array_element_2)))))) (+ (.z (Transformation|GetActorLocation _array_element_2)) 9e+01)) (.rotation (Utilities|Select :Index FormationType :NewEnumerator0 (Transformation|GetWorldTransform (Variables|/Game/Blueprints/Formation/BP_CharacterBattleSpot.BP_CharacterBattleSpot_C|GetFrontlineArrow _array_element_2)) :NewEnumerator1 (Transformation|GetWorldTransform (Variables|/Game/Blueprints/Formation/BP_CharacterBattleSpot.BP_CharacterBattleSpot_C|GetMiddlelineArrow _array_element_2)) :NewEnumerator2 (Transformation|GetWorldTransform (Variables|/Game/Blueprints/Formation/BP_CharacterBattleSpot.BP_CharacterBattleSpot_C|GetBacklineArrow _array_element_2)))) (.scale (Utilities|Select :Index FormationType :NewEnumerator0 (Transformation|GetWorldTransform (Variables|/Game/Blueprints/Formation/BP_CharacterBattleSpot.BP_CharacterBattleSpot_C|GetFrontlineArrow _array_element_2)) :NewEnumerator1 (Transformation|GetWorldTransform (Variables|/Game/Blueprints/Formation/BP_CharacterBattleSpot.BP_CharacterBattleSpot_C|GetMiddlelineArrow _array_element_2)) :NewEnumerator2 (Transformation|GetWorldTransform (Variables|/Game/Blueprints/Formation/BP_CharacterBattleSpot.BP_CharacterBattleSpot_C|GetBacklineArrow _array_element_2))))))
            (goto _label_2 Break)))
        (:Completed
          (return (LocalVariables|GetBattleSpotTransformLocal) FormationType))))))

(fn SpawnEnemies
  (bind _keys (Utilities|Map|Keys (Variables|/Game/Blueprints/Essential/BP_GI_Custom.BP_GI_Custom_C|GetEncounteredEnemies (Variables|Default|GetGame%20Instance%20Reference))))
  (for _array_element _keys
    (bind _returnvalue (Utilities|GetDataTableRow "/Game/Blueprints/DataBases/DT_Enemies.DT_Enemies" (.Value (Utilities|Map|Find (Variables|/Game/Blueprints/Essential/BP_GI_Custom.BP_GI_Custom_C|GetEncounteredEnemies (Variables|Default|GetGame%20Instance%20Reference)) _array_element)))
      (:then
        (bind _returnvalue_2 (Game|SpawnActorfromClass (.EnemyActorClass (Utilities|Struct|BreakS_Enemy _returnvalue)) (.Battle%20Spot%20Transform (BattleBegin|GetProperBattleSpawnTransform false _array_element "NewEnumerator0")) "Undefined" "MultiplyWithRoot" 0 self (Actor|GetComponentbyClass (Components|GetOwner) "/Game/Blueprints/Components/AC_TargetManager.AC_TargetManager_C") true true (.BattleSpotFormationType (BattleBegin|GetProperBattleSpawnTransform false _array_element "NewEnumerator0")) 0))
        (Variables|/Game/Blueprints/Components/AC_Character_BattleStats.AC_Character_BattleStats_C|SetBattleManagerReference (Variables|/Game/Blueprints/Essential/BP_Character_Battle_Base.BP_Character_Battle_Base_C|GetAC_Character_BattleStats _returnvalue_2) self)
        (Default|SetCharacterData (Variables|/Game/Blueprints/Essential/BP_Character_Battle_Base.BP_Character_Battle_Base_C|GetAC_Character_BattleStats _returnvalue_2) (.EnemyDisplayName (Utilities|Struct|BreakS_Enemy _returnvalue)) (.EnemyStats (Utilities|Struct|BreakS_Enemy _returnvalue)) (.Value (Utilities|Map|Find (.EnemyStats (Utilities|Struct|BreakS_Enemy _returnvalue)) "NewEnumerator1")) (.Value (Utilities|Map|Find (.EnemyStats (Utilities|Struct|BreakS_Enemy _returnvalue)) "NewEnumerator2")))
        (Utilities|Array|Add (Variables|BattleinProgress|GetEnemies) _returnvalue_2)))))

(fn GetCharacterwithMaxInitiative
  (for _array_element (Variables|BattleinProgress|GetPlayerCharacters) :!label _label
    (if (>= (Variables|/Game/Blueprints/Components/AC_Character_BattleStats.AC_Character_BattleStats_C|GetCurrentInitiative (Variables|/Game/Blueprints/Essential/BP_Character_Battle_Base.BP_Character_Battle_Base_C|GetAC_Character_BattleStats _array_element)) (Variables|Setup|GetInitiativeNeededToTakeTurn))
      (LocalVariables|SetSuccess?_Local true)
      (LocalVariables|SetCharacterLocal _array_element)
      (goto _label)))
  (if (LocalVariables|GetSuccess?_Local)
    (return (LocalVariables|GetSuccess?_Local) (LocalVariables|GetCharacterLocal))
    (else
      (bind _array_element_2 (Utilities|Array|ForEachLoopwithBreak (Variables|BattleinProgress|GetEnemies) :!label _label_2)
        (:LoopBody
          (if (>= (Variables|/Game/Blueprints/Components/AC_Character_BattleStats.AC_Character_BattleStats_C|GetCurrentInitiative (Variables|/Game/Blueprints/Essential/BP_Character_Battle_Base.BP_Character_Battle_Base_C|GetAC_Character_BattleStats _array_element_2)) (Variables|Setup|GetInitiativeNeededToTakeTurn))
            (LocalVariables|SetSuccess?_Local true)
            (LocalVariables|SetCharacterLocal _array_element_2)
            (goto _label_2 Break)))
        (:Completed
          (return (LocalVariables|GetSuccess?_Local) (LocalVariables|GetCharacterLocal)))))))

(fn StartCharacterTurn
  (params (Charcter :type BP%20Character%20Battle%20Base%20Object%20Reference))
  (bind _output_get (Variables|BattleinProgress|SetCurrentCharacter Charcter))
  (if (not (Variables|/Game/Blueprints/Essential/BP_Character_Battle_Base.BP_Character_Battle_Base_C|GetControlledByBattleAI? _output_get))
    (Variables|/Game/Blueprints/Components/AC_Character_BattleStats.AC_Character_BattleStats_C|SetDefending (Variables|/Game/Blueprints/Essential/BP_Character_Battle_Base.BP_Character_Battle_Base_C|GetAC_Character_BattleStats _output_get) false)
    (bind _characterbattleslotref (Variables|/Game/Blueprints/Components/AC_Character_BattleStats.AC_Character_BattleStats_C|GetCharacterBattleSlotRef (Variables|/Game/Blueprints/Essential/BP_Character_Battle_Base.BP_Character_Battle_Base_C|GetAC_Character_BattleStats _output_get))
      (:then
        (Default|HighlightSlot _characterbattleslotref))
      (:else))
    (else
      (Default|PerformActionbyAI (Variables|BattleinProgress|GetCurrentCharacter)))))

(fn SelectAction
  (params (Action%20Type :type E_ActionType%20Enum :default "NewEnumerator0"))
  (bind _returnvalue (Components|GetOwner))
  (bind _returnvalue_2 (Actor|GetComponentbyClass _returnvalue "/Game/Blueprints/Components/AC_ActionManager.AC_ActionManager_C"))
  (bind _output_get (Variables|Default|SetAction%20Type Action%20Type))
  (switch Utilities|FlowControl|Switch|SwitchonE_ActionType _output_get
    (:NewEnumerator1
      _)
    (:NewEnumerator3
      _)
    (:NewEnumerator5
      _)
    (:NewEnumerator7
      _))
  (Utilities|IsValid _returnvalue_2
    (:Is%20Valid
      (Default|SelectAction _returnvalue_2 (Variables|Default|GetAction%20Type) "None"))))

(fn ShowBattleToolTip
  (params (TooltipText :type Text))
  (bind _foundwidgets (Widget|GetAllWidgetsOfClass "/Game/widgets/Widgets/Battle/WBP_jRPG_BattleInterface.WBP_jRPG_BattleInterface_C" false))
  (Utilities|IsValid (Utilities|Array|Get(acopy) _foundwidgets)
    (:Is%20Valid
      (Rendering|Components|TextRender|SetText (Variables|/Game/widgets/Widgets/Battle/WBP_jRPG_BattleInterface.WBP_jRPG_BattleInterface_C|GetTextBlock_TooltipText (Utilities|Array|Get(acopy) _foundwidgets)) TooltipText)
      (Default|FadeOutTooltipText (Utilities|Array|Get(acopy) _foundwidgets)))))

(fn DisableTargetingandInput
  (bind _returnvalue (Components|GetOwner))
  (bind _returnvalue_2 (Actor|GetComponentbyClass _returnvalue "/Game/Blueprints/Components/AC_TargetManager.AC_TargetManager_C"))
  (Utilities|IsValid _returnvalue_2
    (:Is%20Valid
      (Default|DisableTarget _returnvalue_2)
      (Default|HideTarget _returnvalue_2))))

(fn EndCharacterTurn
  (params (UsedInitiative :type Float%20%28double-precision%29))
  (bind _currentcharacter (Variables|BattleinProgress|GetCurrentCharacter))
  (bind _ac_character_battlestats (Variables|/Game/Blueprints/Essential/BP_Character_Battle_Base.BP_Character_Battle_Base_C|GetAC_Character_BattleStats _currentcharacter))
  (Default|RemoveInitiative _ac_character_battlestats UsedInitiative)
  (BattleInProgress|ActionSelection|HideActionWidget)
  (bind _characterbattleslotref (Variables|/Game/Blueprints/Components/AC_Character_BattleStats.AC_Character_BattleStats_C|GetCharacterBattleSlotRef _ac_character_battlestats)
    (:then
      (Default|UnhighlightSlot _characterbattleslotref)
      (Class|WidgetSwitcher|SetActiveWidgetIndex (Variables|/Game/widgets/Widgets/Battle/WBP_jRPG_ActionsWidget.WBP_jRPG_ActionsWidget_C|GetWidgetSwitcher_Action (Variables|/Game/widgets/Widgets/Battle/WBP_jRPG_BattleInterface.WBP_jRPG_BattleInterface_C|GetWBP_jRPG_ActionsWidget (Variables|Default|GetBattleInterfaceRef)))))
    (:else)))

(fn HideActionWidget
  (bind _battleinterfaceref (Variables|Default|GetBattleInterfaceRef)
    (:then
      (Widget|SetVisibility (Variables|/Game/widgets/Widgets/Battle/WBP_jRPG_BattleInterface.WBP_jRPG_BattleInterface_C|GetWBP_jRPG_ActionsWidget _battleinterfaceref) "Hidden"))
    (:else)))

(fn GoBacktoWorldMap
  (bind _game_instance_reference (Variables|Default|GetGame%20Instance%20Reference))
  (for _array_element (Variables|BattleinProgress|GetPlayerCharacters)
    (bind _structout (Utilities|Struct|SetmembersinS_CharacterStatus (.Value (Utilities|Map|Find (Variables|/Game/Blueprints/Essential/BP_GI_Custom.BP_GI_Custom_C|GetCharactersCollection (Variables|Default|GetGame%20Instance%20Reference)) (Variables|/Game/Blueprints/Components/AC_Character_BattleStats.AC_Character_BattleStats_C|GetCharacterCodedName (Variables|/Game/Blueprints/Essential/BP_Character_Battle_Base.BP_Character_Battle_Base_C|GetAC_Character_BattleStats _array_element)))) (Variables|/Game/Blueprints/Components/AC_Character_BattleStats.AC_Character_BattleStats_C|GetCurrent%20HP (Variables|/Game/Blueprints/Essential/BP_Character_Battle_Base.BP_Character_Battle_Base_C|GetAC_Character_BattleStats _array_element)) (Variables|/Game/Blueprints/Components/AC_Character_BattleStats.AC_Character_BattleStats_C|GetCurrent%20SP (Variables|/Game/Blueprints/Essential/BP_Character_Battle_Base.BP_Character_Battle_Base_C|GetAC_Character_BattleStats _array_element))))
    (Utilities|Map|Add (Variables|/Game/Blueprints/Essential/BP_GI_Custom.BP_GI_Custom_C|GetCharactersCollection (Variables|Default|GetGame%20Instance%20Reference)) (Variables|/Game/Blueprints/Components/AC_Character_BattleStats.AC_Character_BattleStats_C|GetCharacterCodedName (Variables|/Game/Blueprints/Essential/BP_Character_Battle_Base.BP_Character_Battle_Base_C|GetAC_Character_BattleStats _array_element)) _structout))
  (for _array_element_2 (Variables|BattleinProgress|GetDeadPlayerCharacters)
    (bind _structout_2 (Utilities|Struct|SetmembersinS_CharacterStatus (.Value (Utilities|Map|Find (Variables|/Game/Blueprints/Essential/BP_GI_Custom.BP_GI_Custom_C|GetCharactersCollection (Variables|Default|GetGame%20Instance%20Reference)) (Variables|/Game/Blueprints/Components/AC_Character_BattleStats.AC_Character_BattleStats_C|GetCharacterCodedName (Variables|/Game/Blueprints/Essential/BP_Character_Battle_Base.BP_Character_Battle_Base_C|GetAC_Character_BattleStats _array_element_2)))) (Variables|/Game/Blueprints/Components/AC_Character_BattleStats.AC_Character_BattleStats_C|GetCurrent%20HP (Variables|/Game/Blueprints/Essential/BP_Character_Battle_Base.BP_Character_Battle_Base_C|GetAC_Character_BattleStats _array_element_2)) (Variables|/Game/Blueprints/Components/AC_Character_BattleStats.AC_Character_BattleStats_C|GetCurrent%20SP (Variables|/Game/Blueprints/Essential/BP_Character_Battle_Base.BP_Character_Battle_Base_C|GetAC_Character_BattleStats _array_element_2))))
    (Utilities|Map|Add (Variables|/Game/Blueprints/Essential/BP_GI_Custom.BP_GI_Custom_C|GetCharactersCollection (Variables|Default|GetGame%20Instance%20Reference)) (Variables|/Game/Blueprints/Components/AC_Character_BattleStats.AC_Character_BattleStats_C|GetCharacterCodedName (Variables|/Game/Blueprints/Essential/BP_Character_Battle_Base.BP_Character_Battle_Base_C|GetAC_Character_BattleStats _array_element_2)) _structout_2))
  (Variables|/Game/Blueprints/Essential/BP_GI_Custom.BP_GI_Custom_C|SetSpawningAfterBattle? _game_instance_reference true)
  (Game|OpenLevel(byName) (Variables|/Game/Blueprints/Essential/BP_GI_Custom.BP_GI_Custom_C|GetWorldMapName _game_instance_reference)))
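; Character component that holds a jRPG combatant's stats, HP, SP and initiative during battle.
; It creates the character's slot widget in the battle interface and refreshes it as values change.
; Initiative is measured against the battle manager's turn threshold.
; Damage handling includes a Luck-weighted critical roll and defend reduction, while damage, death, healing and initiative loss are reported to the owning actor through messages.
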(event EventBeginPlay
  (bind _asbp_gi_custom (Utilities|Casting|CastToBP_GI_Custom (Game|GetGameInstance) :!label _label)
    (:then
      (Variables|Default|SetGameInstanceReference _asbp_gi_custom))
    (:CastFailed
      (Utilities|FlowControl|Delay 0.1)
      (goto _label))))

(fn SetCharacterData
  (params (CharacterDisplayName :type Text) (CharacterStats :type Map%20of%20E_StatusType%20Enums%20to%20Reals :default "NewEnumerator0") (CurrentHP :type Float%20%28double-precision%29) (CurrentSP :type Float%20%28double-precision%29))
  (Variables|Setup|SetCharacter%20Display%20Name CharacterDisplayName)
  (Variables|Default|SetCharacter%20Stats CharacterStats)
  (Variables|Default|SetCurrent%20HP CurrentHP)
  (Variables|Default|SetCurrent%20SP CurrentSP))

(fn CreateCharacterBattleSlot
  (bind _returnvalue (UserInterface|CreateWidget "/Game/widgets/Widgets/Battle/WBP_jRPG_BattleCharacterSlot.WBP_jRPG_BattleCharacterSlot_C" 0 self))
  (Variables|Reference|SetCharacterBattleSlotRef _returnvalue)
  (Default|UpdateCharacterDisplayName (Variables|Reference|GetCharacterBattleSlotRef) (Variables|Setup|GetCharacter%20Display%20Name))
  (Widget|RefreshHP)
  (Widget|RefreshSP)
  (Initiative||RefreshInitiative)
  (bind _foundwidgets (Widget|GetAllWidgetsOfClass "/Game/widgets/Widgets/Battle/WBP_jRPG_BattleInterface.WBP_jRPG_BattleInterface_C" false))
  (Utilities|IsValid (Utilities|Array|Get(acopy) _foundwidgets)
    (:Is%20Valid
      (Widget|Panel|AddChild (Variables|/Game/widgets/Widgets/Battle/WBP_jRPG_BattleInterface.WBP_jRPG_BattleInterface_C|GetContainer_BattleSlots (Utilities|Array|Get(acopy) _foundwidgets)) (Variables|Reference|GetCharacterBattleSlotRef)))))

(fn AddInitiative
  (params (Amount :type Float%20%28double-precision%29))
  (if (== Amount 0.0)
    (Variables|Default|SetCurrentInitiative (Math|Float|Clamp(Float) (+ (Variables|Default|GetCurrentInitiative) (.Value (Utilities|Map|Find (Variables|Default|GetCharacter%20Stats) "NewEnumerator7"))) 0.0 1e+03))
    (else
      (Variables|Default|SetCurrentInitiative (Math|Float|Clamp(Float) (+ (Variables|Default|GetCurrentInitiative) Amount) 0.0 1e+03))))
  (Initiative||RefreshInitiative))

(fn RefreshHP
  (bind _characterbattleslotref (Variables|Reference|GetCharacterBattleSlotRef)
    (:then
      (Default|UpdateHealthValue _characterbattleslotref (Variables|Default|GetCurrent%20HP) (.Value (Utilities|Map|Find (Variables|Default|GetCharacter%20Stats) "NewEnumerator1"))))
    (:else)))

(fn RefreshSP
  (bind _characterbattleslotref (Variables|Reference|GetCharacterBattleSlotRef)
    (:then
      (Default|UpdateSPValue _characterbattleslotref (Variables|Default|GetCurrent%20SP) (.Value (Utilities|Map|Find (Variables|Default|GetCharacter%20Stats) "NewEnumerator2"))))
    (:else)))

(fn RefreshInitiative
  (bind _battlemanagerreference (Variables|Reference|GetBattleManagerReference)
    (:then
      (bind _characterbattleslotref (Variables|Reference|GetCharacterBattleSlotRef)
        (:then
          (Default|UpdateInitiativeValue _characterbattleslotref (Variables|Default|GetCurrentInitiative) (Variables|/Game/Blueprints/Components/AC_BattleManager.AC_BattleManager_C|GetInitiativeNeededToTakeTurn _battlemanagerreference)))
        (:else)))
    (:else)))

(fn RemoveInitiative
  (params (Amount :type Float%20%28double-precision%29))
  (Variables|Default|SetCurrentInitiative (Math|Float|Clamp(Float) (- (Variables|Default|GetCurrentInitiative) Amount) 0.0 1e+03))
  (Initiative||RefreshInitiative))

(fn ReceiveDamage
  (params (Damage :type Float%20%28double-precision%29) (Luck :type Float%20%28double-precision%29) (CRIT :type Float%20%28double-precision%29))
  (LocalVariables|SetDamageLocal Damage)
  (if (> (Variables|Default|GetCurrent%20HP) 0.0)
    (bind _output_get (LocalVariables|SetCirtical?Local (Math|Random|RandomBoolwithWeight (/ Luck 1e+02))))
    (if _output_get
      (LocalVariables|SetDamageLocal (* (LocalVariables|GetDamageLocal) (/ CRIT 1e+02))))
    (bind _output_get_2 (LocalVariables|SetDamageLocal (.Value (Utilities|Map|Find (Variables|Default|GetCharacter%20Stats) "NewEnumerator11"))))
    (bind _damagedealt (Damage|CalculateDefendwithFleeReduction _output_get_2))
    (LocalVariables|SetDamageLocal (Math|Conversions|ToFloat(Integer) (Math|Float|Truncate (Math|Float|Clamp(Float) _damagedealt 1.0 9999.0))))
    (Variables|Default|SetCurrent%20HP (Math|Float|Clamp(Float) (- (Variables|Default|GetCurrent%20HP) (LocalVariables|GetDamageLocal)) 0.0 (.Value (Utilities|Map|Find (Variables|Default|GetCharacter%20Stats) "NewEnumerator1"))))
    (Utilities|FlowControl|Sequence
      (:then_0
        (Class|BPIBattleCommunication|OnDamageReceived(Message) (Components|GetOwner) (LocalVariables|GetDamageLocal) (LocalVariables|GetCirtical?Local)))
      (:then_1
        (Widget|RefreshHP))
      (:then_2
        (if (== (Variables|Default|GetCurrent%20HP) 0.0)
          (Class|BPIBattleCommunication|OnDeath(Message) (Components|GetOwner)))))))

(fn CalculateDefendwithFleeReduction
  (params (DamageInput :type Float%20%28double-precision%29))
  (if (Variables|Default|GetDefending)
    (return (* DamageInput 0.75))
    (else
      (return DamageInput))))

(fn ReduceInitiative
  (params (Amount :type Float%20%28double-precision%29))
  (Variables|Default|SetCurrentInitiative (Math|Float|Clamp(Float) (- (Variables|Default|GetCurrentInitiative) Amount) 0.0 (Variables|/Game/Blueprints/Components/AC_BattleManager.AC_BattleManager_C|GetInitiativeNeededToTakeTurn (Variables|Reference|GetBattleManagerReference))))
  (Class|BPIBattleCommunication|OnInitiativeReduced(Message) (Components|GetOwner) Amount)
  (Initiative||RefreshInitiative))

(fn ReduceHP
  (params (Amount :type Float%20%28double-precision%29))
  (Variables|Default|SetCurrent%20HP (- (Variables|Default|GetCurrent%20HP) Amount))
  (Widget|RefreshHP))

(fn ReduceSP
  (params (Amount :type Float%20%28double-precision%29))
  (Variables|Default|SetCurrent%20SP (- (Variables|Default|GetCurrent%20SP) Amount))
  (Widget|RefreshSP))

(fn RecoverHP
  (params (RecoveryAmount :type Float%20%28double-precision%29))
  (Variables|Default|SetCurrent%20HP (Math|Float|Clamp(Float) (+ RecoveryAmount (Variables|Default|GetCurrent%20HP)) 0.0 (.Value (Utilities|Map|Find (Variables|Default|GetCharacter%20Stats) "NewEnumerator1"))))
  (Widget|RefreshHP)
  (Class|BPIBattleCommunication|OnHealed(Message) (Components|GetOwner) RecoveryAmount false))

(fn RecoverSP
  (params (RecoveryAmount :type Float%20%28double-precision%29))
  (Variables|Default|SetCurrent%20SP (Math|Float|Clamp(Float) (+ RecoveryAmount (Variables|Default|GetCurrent%20SP)) 0.0 (.Value (Utilities|Map|Find (Variables|Default|GetCharacter%20Stats) "NewEnumerator2"))))
  (Widget|RefreshSP)
  (Class|BPIBattleCommunication|OnHealed(Message) (Components|GetOwner) RecoveryAmount true))

(fn Reincarnation
  (params (HP%20Amount :type Float%20%28double-precision%29))
  (bind _output_get (Variables|Default|SetCurrent%20HP (Math|Float|Clamp(Float) HP%20Amount 0.0 (.Value (Utilities|Map|Find (Variables|Default|GetCharacter%20Stats) "NewEnumerator1")))))
  (Widget|RefreshHP)
  (Class|BPIBattleCommunication|OnHealed(Message) (Components|GetOwner) _output_get false))
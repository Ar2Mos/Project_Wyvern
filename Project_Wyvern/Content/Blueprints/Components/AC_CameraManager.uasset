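; Camera manager component that flies a spawned camera along spline paths defined by BP_CameraPath actors.
; At BeginPlay it maps paths by ID, makes the camera the first player's view target and can auto-start a default looping path.
; Tick advances distance at constant speed, looping or stopping at the end, and aims the camera at the path's focus point.
; SetNewDynamicPath switches paths, optionally randomizing start distance or relocating the path.
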(event EventBeginPlay
  (Utilities|FlowControl|Sequence
    (:then_0
      (bind _outactors (Actor|GetAllActorsOfClass "/Game/Blueprints/Other/Battle/BP_CameraPath.BP_CameraPath_C"))
      (for _array_element _outactors
        (Utilities|Map|Add (Variables|References|GetDynamicCameraPath) (Variables|/Game/Blueprints/Other/Battle/BP_CameraPath.BP_CameraPath_C|GetPathID _array_element) _array_element)))
    (:then_1
      (bind _returnvalue (Game|SpawnActorfromClass "/Script/Engine.CameraActor" (Math|Transform|MakeTransform "0, 0, 0" "0, 0, 0" "1.000000,1.000000,1.000000") "Undefined" "MultiplyWithRoot" 0 0))
      (bind _output_get (Variables|References|SetCameraActor _returnvalue))
      (Game|Player|SetViewTargetwithBlend (Game|GetPlayerController 0) _output_get 0.0 "VTBlend_Linear" 0.0 false))
    (:then_2
      (if (Variables|General|GetUseAutoCameraManagement?)
        (CallFunction|SetNewDynamicPath (Variables|General|GetDefaultCameraID) true true false "0, 0, 0")))))

(event EventTick
  (params (DeltaSeconds :type Float%20%28single-precision%29))
  (Utilities|IsValid (Variables|PathManagement|GetActiveCamera)
    (:Is%20Valid
      (if (>= (Variables|PathManagement|GetPathDistance) (Spline|GetSplineLength (Variables|/Game/Blueprints/Other/Battle/BP_CameraPath.BP_CameraPath_C|GetSpline (Variables|PathManagement|GetActiveCamera))))
        (if (Variables|PathManagement|GetLoopEnabled)
          (Variables|PathManagement|SetPathDistance 0.0)
          (bind _output_get (Variables|PathManagement|SetPathDistance (+ (Variables|PathManagement|GetPathDistance) (* (Variables|PathManagement|GetSpeed) (Utilities|Time|GetWorldDeltaSeconds))) :!label _label))
          (CallFunction|UpdateCameraLocationandRotation _output_get))
        (else
          (goto _label))))))

(fn SetNewDynamicPath
  (params (PathID :type Name) (RandomStartDistance :type Boolean) (Loop :type Boolean) (UpdatePathLocation :type Boolean) (NewLocation :type Vector))
  (bind _dynamiccamerapath (Variables|References|GetDynamicCameraPath))
  (bind (_value _returnvalue) (Utilities|Map|Find _dynamiccamerapath PathID))
  (Variables|PathManagement|SetLoopEnabled Loop)
  (if _returnvalue
    (Variables|PathManagement|SetActiveCamera _value)
    (Variables|PathManagement|SetPathDistance (Math|Float|SelectFloat (* (Math|Random|RandomFloatinRange 0.0 0.8) (Spline|GetSplineLength (Variables|/Game/Blueprints/Other/Battle/BP_CameraPath.BP_CameraPath_C|GetSpline (Variables|PathManagement|GetActiveCamera)))) 0.0 RandomStartDistance))
    (if UpdatePathLocation
      (Transformation|SetActorLocation (Variables|PathManagement|GetActiveCamera) NewLocation false false))
    (else
      (Development|PrintString (Utilities|String|Append "Couldn't find camera path with ID: " (Utilities|String|ToString(Name) PathID))))))

(fn UpdateCameraLocationandRotation
  (params (PathTime :type Float%20%28double-precision%29))
  (Utilities|IsValid (Variables|PathManagement|GetActiveCamera)
    (:Is%20Valid
      (bind _cameraactor (Variables|References|GetCameraActor)
        (:then
          (Transformation|SetActorLocation _cameraactor (Default|GetPathLocationatDistance (Variables|PathManagement|GetActiveCamera) PathTime) false false)
          (Transformation|SetActorRotation (Variables|References|GetCameraActor) (Math|Rotator|FindLookatRotation (Transformation|GetActorLocation (Variables|References|GetCameraActor)) (Default|GetCameraFocusPoint (Variables|PathManagement|GetActiveCamera)))))
        (:else)))))
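; Interactable door that consumes a Key from the player's inventory to advance to the boss level.
; On interaction it loops over the game instance's inventory, showing a missing-key popup for each non-matching item.
; A match removes the key through the inventory manager, passing the found item index as the amount, increments CurrentFloor and opens Map_World_Boss.
; An every-third-floor boss check with regular-level loading is left disconnected.
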(event EventBeginPlay
  (|CallParentFunction) ; This node is disabled and will not be called.\nDrag off pins to build functionality.
)

(event Collision|EventActorBeginOverlap
  (params (OtherActor :type Actor%20Object%20Reference)))

(event EventTick
  (params (DeltaSeconds :type Float%20%28single-precision%29)))

(event EventOnInteractionRequested
  (params (InteractingWorldCharacter :type BP%20World%20Character%20Object%20Reference))
  (bind _playercontroller (Variables|/Game/Blueprints/Essential/BP_WorldCharacter.BP_WorldCharacter_C|GetPlayerController InteractingWorldCharacter))
  (Utilities|IsValid InteractingWorldCharacter
    (:Is%20Valid
      (bind _asbp_gi_custom (Utilities|Casting|CastToBP_GI_Custom (Game|GetGameInstance)))
      (bind _output_get (Variables|Default|SetGameInstanceRef _asbp_gi_custom))
      (for _array_element (Variables|/Game/Blueprints/Essential/BP_GI_Custom.BP_GI_Custom_C|GetInventory _output_get)
        (if (== (.ItemCodedName (Utilities|Struct|BreakS_ItemData (.ItemsData (Utilities|Struct|BreakS_Items_Dynamic _array_element)))) (Variables|Default|GetKey))
          (CallFunction|RemoveKeysfromInventory (Variables|/Game/Blueprints/Essential/Controller/BP_PlayerController_World.BP_PlayerController_World_C|GetAC_InventoryManager _playercontroller) (Variables|Default|GetKey))
          (bind _result (Math|Integer|IncrementInt (Variables|/Game/Blueprints/Essential/BP_GI_Custom.BP_GI_Custom_C|GetCurrentFloor _output_get))
            (:%20%20
              (Game|OpenLevel(byName) "Map_World_Boss")))
          (else
            (Default|ShowInteractionPopUp _playercontroller "You didn't have a key")))))))

(fn ConstructionScript
  (|CallParentFunction))

(fn RemoveKeysfromInventory
  (params (Inventory%20Manager :type AC%20Inventory%20Manager%20Object%20Reference) (ItemCodedName :type Name))
  (bind (_success_ _isitemfullystack_ _itemindex) (Default|CheckifThereIsIteminInven Inventory%20Manager ItemCodedName))
  (if _success_
    (Default|RemoveItemFormInventory Inventory%20Manager ItemCodedName _itemindex)))
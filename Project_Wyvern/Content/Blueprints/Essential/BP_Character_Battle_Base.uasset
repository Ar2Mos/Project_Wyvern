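; Base character for turn-based battles, handling mouse targeting, action dispatch and death state.
; Capsule hover shows or hides the target through the target manager, and clicking a targeted character asks the battle manager to execute the action.
; ExecuteAction routes each action type to empty, overridable events.
; The stats component handles attack damage and defending, while the AI turn only lowers its own initiative and advances everyone's through the battle manager.
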(event OnBeginCursorOver(CapsuleComponent)
  (params (TouchedComponent :type Primitive%20Component%20Object%20Reference))
  (bind _targetmanagerreference (Variables|Default|GetTargetManagerReference)
    (:then
      (if (Variables|/Game/Blueprints/Components/AC_TargetManager.AC_TargetManager_C|GetTargetEnabled? _targetmanagerreference)
        (Default|ShowTarget _targetmanagerreference self)))
    (:else)))

(event OnClicked(CapsuleComponent)
  (params (TouchedComponent :type Primitive%20Component%20Object%20Reference) (ButtonPressed :type Key%20Structure :default "None"))
  (bind _targetmanagerreference (Variables|Default|GetTargetManagerReference)
    (:then
      (if (Variables|/Game/Blueprints/Components/AC_TargetManager.AC_TargetManager_C|GetTargetEnabled? _targetmanagerreference)
        _
        (else
          _))
      (if (Utilities|Array|ContainsItem (Variables|/Game/Blueprints/Components/AC_TargetManager.AC_TargetManager_C|GetTargetedCharacters _targetmanagerreference) self)
        (bind _battlemanagerreference (Variables|Default|GetBattleManagerReference)
          (:then
            (Default|RequestActionExecution _battlemanagerreference (Variables|/Game/Blueprints/Components/AC_TargetManager.AC_TargetManager_C|GetTargetedCharacters _targetmanagerreference)))
          (:else))))
    (:else)))

(event OnEndCursorOver(CapsuleComponent)
  (params (TouchedComponent :type Primitive%20Component%20Object%20Reference))
  (bind _targetmanagerreference (Variables|Default|GetTargetManagerReference)
    (:then
      (if (Variables|/Game/Blueprints/Components/AC_TargetManager.AC_TargetManager_C|GetTargetEnabled? _targetmanagerreference)
        (Default|HideTarget _targetmanagerreference)))
    (:else)))

(event EventOnDeath
  (Variables|Battle|SetDead? true)
  (Variables|/Game/Blueprints/Components/AC_Character_BattleStats.AC_Character_BattleStats_C|SetDefending (Variables|Default|GetAC_Character_BattleStats) false)
  (Animation|StopAnimMontage (Animation|GetCurrentMontage :!class /Script/Engine.Character)))

(event Custom|ExecuteAction
  (params (ActionType :type E_ActionType%20Enum :default "NewEnumerator0") (SecondaryActionName :type Name))
  (switch Utilities|FlowControl|Switch|SwitchonE_ActionType ActionType
    (:NewEnumerator1
      (CallFunction|ExecuteAttackAction))
    (:NewEnumerator2
      (CallFunction|ExecuteMagicAction SecondaryActionName))
    (:NewEnumerator3
      (CallFunction|ExecuteDefendAction))
    (:NewEnumerator4
      (CallFunction|ExecuteItemAction SecondaryActionName))
    (:NewEnumerator5
      (CallFunction|ExecuteFleeAction))
    (:NewEnumerator6
      (CallFunction|ExecuteMoveAction SecondaryActionName))
    (:NewEnumerator7
      (CallFunction|ExecuteSpacialMoveAction SecondaryActionName))))

(event Custom|ExecuteSpacialMoveAction
  (params (SpacialMoveName :type Name)))

(event Custom|ExecuteDefendAction)

(event Custom|ExecuteItemAction
  (params (ItemName :type Name)))

(event Custom|ExecuteFleeAction)

(event Custom|ExecuteMagicAction
  (params (MagicName :type Name)))

(event Custom|ExecuteAttackAction)

(event Custom|ExecuteMoveAction
  (params (MoveName :type Name)))

(fn ConstructionScript)

(fn PerformActionbyAI
  (Default|AddInitiative (Variables|Default|GetAC_Character_BattleStats) -9e+02)
  (Default|AddInitativetoAllChars (Variables|Default|GetBattleManagerReference)))

(fn ApplyAttackEffect
  (bind _ac_character_battlestats (Variables|Default|GetAC_Character_BattleStats))
  (bind _character_stats (Variables|/Game/Blueprints/Components/AC_Character_BattleStats.AC_Character_BattleStats_C|GetCharacter%20Stats _ac_character_battlestats))
  (for _array_element (Variables|Battle|GetTargetedCharacters)
    (Utilities|IsValid _array_element
      (:Is%20Valid
        (Default|ReceiveDamage (Variables|BP_Character_Battle_Base_C|GetAC_Character_BattleStats _array_element) (.Value (Utilities|Map|Find _character_stats "NewEnumerator9")) (.Value (Utilities|Map|Find _character_stats "NewEnumerator8")) (.Value (Utilities|Map|Find _character_stats "NewEnumerator10")))))))

(fn GetCharacterJobClass
  (return (Variables|Battle|GetJobClass)))

(fn GetIsDead
  (return (Variables|Battle|GetDead?)))

(fn GetIsDefending
  (bind _ac_character_battlestats (Variables|Default|GetAC_Character_BattleStats)
    (:then
      (return (Variables|/Game/Blueprints/Components/AC_Character_BattleStats.AC_Character_BattleStats_C|GetDefending _ac_character_battlestats)))
    (:else
      (return false))))
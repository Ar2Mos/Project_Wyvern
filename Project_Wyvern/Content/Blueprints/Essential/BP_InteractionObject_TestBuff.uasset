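; BP_InteractionObject_TestBuff is a single-use interaction object that opens the WB_Roguelike screen for the character who interacts with it.
; On an interaction request from a valid character, it proceeds only if its object interaction state is false.
; It switches that player to UI-only input with a visible cursor, adds the widget to the viewport, then destroys itself.
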(event EventBeginPlay
  (|CallParentFunction) ; This node is disabled and will not be called.\nDrag off pins to build functionality.
)

(event Collision|EventActorBeginOverlap
  (params (OtherActor :type Actor%20Object%20Reference)))

(event EventTick
  (params (DeltaSeconds :type Float%20%28single-precision%29)))

(event EventOnInteractionRequested
  (params (InteractingWorldCharacter :type BP%20World%20Character%20Object%20Reference))
  (bind _playercontroller (Variables|/Game/Blueprints/Essential/BP_WorldCharacter.BP_WorldCharacter_C|GetPlayerController InteractingWorldCharacter))
  (Utilities|IsValid InteractingWorldCharacter
    (:Is%20Valid
      (if (not (CallFunction|GetObjectInteractionState))
        (Input|SetInputModeUIOnly _playercontroller 0 "DoNotLock" false)
        (Variables|/Script/Engine.PlayerController|SetbShowMouseCursor _playercontroller true)
        (bind _returnvalue (UserInterface|CreateWidget "/Game/widgets/Widgets/Roguelike/WB_Roguelike.WB_Roguelike_C" _playercontroller))
        (UserInterface|Viewport|AddtoViewport _returnvalue 0)
        (Actor|DestroyActor)))))

(fn ConstructionScript
  (|CallParentFunction))
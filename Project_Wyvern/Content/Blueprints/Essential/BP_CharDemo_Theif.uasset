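; Demo Thief player character for turn-based battles, built on Paper2D flipbooks and a battle stats component.
; Its attack action shows a tooltip, ends the turn, then after a short delay damages a random entry among its targets and resumes battle.
; Death and resurrection events update the Dead flag and notify the battle manager, while damage events defer to the parent.
; AttackUpdate always switches to the attack flipbook, as its condition is hardcoded true.
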(event EventBeginPlay
  (|CallParentFunction) ; This node is disabled and will not be called.\nDrag off pins to build functionality.
)

(event Collision|EventActorBeginOverlap
  (params (OtherActor :type Actor%20Object%20Reference))
  (|CallParentFunction OtherActor) ; This node is disabled and will not be called.\nDrag off pins to build functionality.
)

(event EventTick
  (params (DeltaSeconds :type Float%20%28single-precision%29))
  (|CallParentFunction DeltaSeconds) ; This node is disabled and will not be called.\nDrag off pins to build functionality.
)

(event EventOnDeath
  (Variables|/Game/Blueprints/Components/AC_Character_BattleStats.AC_Character_BattleStats_C|SetDefending (Variables|Default|GetAC_Character_BattleStats) false)
  (Variables|Default|SetDead? true)
  (Audio|Components|Audio|Stop (Variables|Default|GetPaperFlipbook))
  (bind _battlemanagerreference (Variables|Default|GetBattleManagerReference)
    (:then
      (Default|OnPlayerCharacterKilled _battlemanagerreference self))
    (:else)))

(event EventOnDamageReceived
  (params (Damage :type Float%20%28double-precision%29) (Critical? :type Boolean))
  ;[1 1 1] Parrent : Damage Pop up
  (|CallParentFunction Damage Critical?))

(event EventOnResurrected
  (params (HealAmount :type Float%20%28double-precision%29))
  (Variables|Default|SetDead? false)
  (bind _battlemanagerreference (Variables|Default|GetBattleManagerReference)
    (:then
      (Default|OnPlayerCharacterReincarnation _battlemanagerreference self))
    (:else)))

(event EventExecuteAttackAction
  (bind _ac_character_battlestats (Variables|Default|GetAC_Character_BattleStats))
  (bind _ac_character_battlestats_2 (Variables|Default|GetAC_Character_BattleStats))
  (bind _character_stats (Variables|/Game/Blueprints/Components/AC_Character_BattleStats.AC_Character_BattleStats_C|GetCharacter%20Stats _ac_character_battlestats))
  (bind _targetedcharacter (Variables|/Game/Blueprints/Components/AC_Character_BattleStats.AC_Character_BattleStats_C|GetTargetedCharacter _ac_character_battlestats_2))
  (bind _battlemanagerreference (Variables|Default|GetBattleManagerReference)
    (:then
      (Default|ShowBattleToolTip _battlemanagerreference (Utilities|Text|FormatText "{name} attacks" (Variables|/Game/Blueprints/Components/AC_Character_BattleStats.AC_Character_BattleStats_C|GetCharacter%20Display%20Name (Variables|Default|GetAC_Character_BattleStats))))
      (Default|EndCharacterTurn (Variables|Default|GetBattleManagerReference) 1e+03)
      (Utilities|FlowControl|Delay 0.3)
      (bind _output_get (Variables|Default|SetTargeted (Utilities|Array|Get(acopy) _targetedcharacter (Math|Random|RandomIntegerinRange 0 (- (Utilities|Array|Length _targetedcharacter) 1)))))
      (Default|ReceiveDamage (Variables|/Game/Blueprints/Essential/BP_Character_Battle_Base.BP_Character_Battle_Base_C|GetAC_Character_BattleStats _output_get) (.Value (Utilities|Map|Find _character_stats "NewEnumerator9")) (.Value (Utilities|Map|Find _character_stats "NewEnumerator8")) (.Value (Utilities|Map|Find _character_stats "NewEnumerator10")))
      (Development|PrintString (Utilities|String|ToString(Float) (Variables|/Game/Blueprints/Components/AC_Character_BattleStats.AC_Character_BattleStats_C|GetCurrent%20HP (Variables|/Game/Blueprints/Essential/BP_Character_Battle_Base.BP_Character_Battle_Base_C|GetAC_Character_BattleStats _output_get))))
      (bind _battlemanagerreference_2 (Variables|/Game/Blueprints/Components/AC_Character_BattleStats.AC_Character_BattleStats_C|GetBattleManagerReference (Variables|Default|GetAC_Character_BattleStats))
        (:then
          (Default|ResumeBattle _battlemanagerreference_2))
        (:else)))
    (:else)))

(fn ConstructionScript
  (|CallParentFunction))

(fn AttackUpdate
  (if true
    (Sprite|SetFlipbook (Variables|Default|GetPaperFlipbook) "/Game/Sprite/thief/thief_attack1.thief_attack1")
    (Development|PrintString "attack")
    (else
      (Sprite|SetFlipbook (Variables|Default|GetPaperFlipbook) "/Game/Sprite/thief/thief_idle.thief_idle"))))

(fn GetIsAttacking
  (return (Variables|Default|GetAttack?)))
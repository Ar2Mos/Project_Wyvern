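; BP_DEMO_Slime is a demo slime enemy for the turn-based battle system, implementing the AI's action as a simple attack.
; On its turn it shows an attack tooltip, ends its turn through the battle manager, then after a short delay damages a random player character using its damage, luck and crit stats.
; It plays the attack flipbook, waits, resumes the battle and prints one of its stats.
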(event EventPerformActionbyAI
  (bind _battlemanagerreference (Variables|Default|GetBattleManagerReference))
  (bind _ac_character_battlestats (Variables|Default|GetAC_Character_BattleStats))
  (bind _battlemanagerreference_2 (Variables|Default|GetBattleManagerReference))
  (bind _playercharacters (Variables|/Game/Blueprints/Components/AC_BattleManager.AC_BattleManager_C|GetPlayerCharacters _battlemanagerreference))
  (bind _character_stats (Variables|/Game/Blueprints/Components/AC_Character_BattleStats.AC_Character_BattleStats_C|GetCharacter%20Stats _ac_character_battlestats))
  (Default|ShowBattleToolTip _battlemanagerreference_2 (Utilities|Text|FormatText "{name} attacks" (Variables|/Game/Blueprints/Components/AC_Character_BattleStats.AC_Character_BattleStats_C|GetCharacter%20Display%20Name (Variables|Default|GetAC_Character_BattleStats))))
  (Default|EndCharacterTurn _battlemanagerreference_2 1e+03)
  (Utilities|FlowControl|Delay 0.25)
  (bind _output_get (Variables|Default|SetTargeted (Utilities|Array|Get(acopy) _playercharacters (Math|Random|RandomIntegerinRange 0 (- (Utilities|Array|Length _playercharacters) 1)))))
  (Default|ReceiveDamage (Variables|/Game/Blueprints/Essential/BP_Character_Battle_Base.BP_Character_Battle_Base_C|GetAC_Character_BattleStats _output_get) (.Value (Utilities|Map|Find _character_stats "NewEnumerator9")) (.Value (Utilities|Map|Find _character_stats "NewEnumerator8")) (.Value (Utilities|Map|Find _character_stats "NewEnumerator10")))
  (Sprite|SetFlipbook (Variables|Default|GetPaperFlipbook) "/Game/Sprite/Slime/slime_attack_L1.slime_attack_L1")
  (Utilities|FlowControl|Delay 1.0)
  (Default|ResumeBattle (Variables|Default|GetBattleManagerReference))
  (Development|PrintString (Utilities|String|ToString(Float) (.Value (Utilities|Map|Find _character_stats "NewEnumerator1")))))

(fn ConstructionScript
  (|CallParentFunction))
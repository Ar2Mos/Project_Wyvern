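; Lootable chest interaction object that gives the interacting character the items in its ItemInChest map, or reports it empty if its interaction state is set.
; Looting adds each entry to the player's inventory manager, shows a popup of DT_Items display names with amounts, and moves the lid open.
; It then writes the current interaction state back unchanged under a test comment, and the state-loaded event is empty.
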(event EventBeginPlay
  (|CallParentFunction) ; This node is disabled and will not be called.\nDrag off pins to build functionality.
)

(event Collision|EventActorBeginOverlap
  (params (OtherActor :type Actor%20Object%20Reference)))

(event EventTick
  (params (DeltaSeconds :type Float%20%28single-precision%29)))

(event EventOnObjectInteractionStateLoaded
  (params (InteractionState :type Boolean)))

(event EventOnInteractionRequested
  (params (InteractingWorldCharacter :type BP%20World%20Character%20Object%20Reference))
  (bind _playercontroller (Variables|/Game/Blueprints/Essential/BP_WorldCharacter.BP_WorldCharacter_C|GetPlayerController InteractingWorldCharacter))
  (bind _chest_lit (Variables|Default|GetChest_Lit))
  (Utilities|IsValid InteractingWorldCharacter
    (:Is%20Valid
      (if (CallFunction|GetObjectInteractionState)
        (Default|ShowInteractionPopUp _playercontroller "Chest is empty.")
        (else
          (CallFunction|AddItemsfromChesttoInventory (Variables|/Game/Blueprints/Essential/Controller/BP_PlayerController_World.BP_PlayerController_World_C|GetAC_InventoryManager _playercontroller))
          (Default|ShowInteractionPopUp _playercontroller (CallFunction|ConstructInteractionPopUpText))
          (CallFunction|SetObjectInteractionState (CallFunction|GetObjectInteractionState))
          (Transformation|SetRelativeRotation _chest_lit "90.000000,0.000000,0.000000" false false)
          (Transformation|SetRelativeLocation _chest_lit "10.000000,0.000000,80.000000" false false))))))

(fn ConstructionScript
  (|CallParentFunction))

(fn ConstructInteractionPopUpText
  (bind _iteminchest (Variables|Default|GetItemInChest))
  (bind _keys (Utilities|Map|Keys _iteminchest))
  (for _array_element _keys
    (bind _returnvalue (Utilities|GetDataTableRow "/Game/Blueprints/DataBases/DT_Items.DT_Items" _array_element)
      (:then
        (LocalVariables|SetPopUpTextLocal (Utilities|Text|FormatText "{current text}{row to add}" (LocalVariables|GetPopUpTextLocal) (Utilities|Text|FormatText "{item name} x {amount}" (.ItemDisplayName (Utilities|Struct|BreakS_ItemData _returnvalue)) (.Value (Utilities|Map|Find _iteminchest _array_element))))))))
  (LocalVariables|SetPopUpTextLocal (Utilities|Text|FormatText "{current text}." (LocalVariables|GetPopUpTextLocal)))
  (return (LocalVariables|GetPopUpTextLocal)))

(fn AddItemsfromChesttoInventory
  (params (InventoryManager :type AC%20Inventory%20Manager%20Object%20Reference))
  (bind _keys (Utilities|Map|Keys (Variables|Default|GetItemInChest)))
  (for _array_element _keys
    (Default|AddItemtoInventory InventoryManager _array_element (.Value (Utilities|Map|Find (Variables|Default|GetItemInChest) _array_element)))))
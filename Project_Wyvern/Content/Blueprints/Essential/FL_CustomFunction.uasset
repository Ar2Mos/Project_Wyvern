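; Blueprint function library of shared RPG helpers for leveling, UI display and map travel.
; An experience helper reads the next level's row in DT_LevelTable and returns the clamped amount still needed.
; Select-based lookups convert rarity, item, action and stat enums into colors, icons or display text.
; ChangeMap stores the map and spawn point names in BP_GI_Custom before opening the level by name.
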(fn GetExperienceNeededtoNextLevel
  (params (Current%20Level :type Integer) (Current%20EXP :type Integer))
  (bind _returnvalue (Utilities|GetDataTableRow "/Game/Blueprints/DataBases/DT_LevelTable.DT_LevelTable" (Utilities|String|StringToName (Utilities|String|ToString(Integer) (+ Current%20Level 1))))
    (:then
      (return (Math|Integer|Clamp(Integer) (- (Utilities|Struct|BreakS_LevelTables _returnvalue) Current%20EXP) 0 (Utilities|Struct|BreakS_LevelTables _returnvalue))))))

(fn RaritytoColor
  (params (Raritiy :type E_RarityType%20Enum :default "NewEnumerator0"))
  (return (Utilities|Select :Index Raritiy :NewEnumerator0 "(R=0.208333,G=0.208333,B=0.208333,A=1.000000)" :NewEnumerator1 "(R=1.000000,G=1.000000,B=1.000000,A=1.000000)" :NewEnumerator2 "(R=0.107261,G=0.281182,B=1.000000,A=1.000000)" :NewEnumerator3 "(R=1.000000,G=0.038389,B=0.844122,A=1.000000)" :NewEnumerator4 "(R=1.000000,G=0.691462,B=0.075730,A=1.000000)" :NewEnumerator5 "(R=1.000000,G=0.044178,B=0.000000,A=1.000000)")))

(fn ItemTypetoImage
  (params (Item%20Type :type E_ItemType%20Enum :default "NewEnumerator0"))
  (return (Utilities|Select :Index Item%20Type :NewEnumerator0 "/Game/Sprite/UI/Circle_ICON_Layout.Circle_ICON_Layout" :NewEnumerator1 "/Game/Sprite/UI/sub/W_Dagger005.W_Dagger005" :NewEnumerator2 "/Game/Sprite/UI/sub/A_Armor04.A_Armor04" :NewEnumerator3 "/Game/Sprite/UI/sub/C_Elm03.C_Elm03" :NewEnumerator4 "/Game/Sprite/UI/sub/C_Hat01.C_Hat01" :NewEnumerator5 "/Game/Sprite/UI/sub/A_Shoes01.A_Shoes01" :NewEnumerator6 "/Game/Sprite/UI/sub/Ac_Ring04.Ac_Ring04" :NewEnumerator7 "/Game/Sprite/UI/sub/Ac_Necklace02.Ac_Necklace02" :NewEnumerator10 "/Game/Sprite/UI/sub/I_Scroll02.I_Scroll02" :NewEnumerator8 "/Game/Sprite/UI/sub/P_Red03.P_Red03" :NewEnumerator9 "/Game/Sprite/UI/sub/I_Key03.I_Key03")))

(fn ActionTypetoText
  (params (Action%20Type :type E_ActionType%20Enum :default "NewEnumerator0"))
  (return (Utilities|Select :Index Action%20Type :NewEnumerator0 "" :NewEnumerator1 "Attack" :NewEnumerator2 "Magic" :NewEnumerator3 "Defend" :NewEnumerator4 "Items" :NewEnumerator5 "Flee" :NewEnumerator6 "Moves" :NewEnumerator7 "Spacial Move")))

(fn StatTypetoText
  (params (StatType :type E_StatusType%20Enum :default "NewEnumerator0"))
  (return (Utilities|Select :Index StatType :NewEnumerator0 "" :NewEnumerator1 "HP" :NewEnumerator2 "SP" :NewEnumerator3 "STR" :NewEnumerator4 "AGI" :NewEnumerator5 "VIT" :NewEnumerator6 "INT" :NewEnumerator7 "DEX" :NewEnumerator8 "LUK" :NewEnumerator9 "ATK" :NewEnumerator10 "CRT" :NewEnumerator11 "FLEE")))

(fn ItemSubtypetoText
  (params (StatType :type E_SubItemType%20Enum :default "NewEnumerator0"))
  (return (Utilities|Select :Index StatType :NewEnumerator0 "" :NewEnumerator1 "Sword" :NewEnumerator2 "Staff" :NewEnumerator3 "Bow" :NewEnumerator4 "Shield" :NewEnumerator5 "Dagge" :NewEnumerator6 "Heavy Protection" :NewEnumerator7 "Cloth Protection" :NewEnumerator8 "Robe Protection" :NewEnumerator9 "Ring" :NewEnumerator11 "Necklance" :NewEnumerator12 "Medicine")))

(fn RaritytoText
  (params (Raritiy :type E_RarityType%20Enum :default "NewEnumerator0"))
  (return (Utilities|Select :Index Raritiy :NewEnumerator0 "Uncommon" :NewEnumerator1 "Common" :NewEnumerator2 "Rare" :NewEnumerator3 "Mystic" :NewEnumerator4 "Epic" :NewEnumerator5 "Legendary")))

(fn ChangeMap
  (params (MapName :type Name) (SpawnPointName :type Name))
  (bind _asbp_gi_custom (Utilities|Casting|CastToBP_GI_Custom (Game|GetGameInstance)))
  (Variables|/Game/Blueprints/Essential/BP_GI_Custom.BP_GI_Custom_C|SetWorldMapSpawnPointName _asbp_gi_custom SpawnPointName)
  (Variables|/Game/Blueprints/Essential/BP_GI_Custom.BP_GI_Custom_C|SetWorldMapName _asbp_gi_custom MapName)
  (Game|OpenLevel(byName) _asbp_gi_custom MapName))
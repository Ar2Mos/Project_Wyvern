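; BP_Controller_Battle is the player controller for battles, showing the mouse cursor and accepting both game and UI input.
; On BeginPlay it waits briefly, then has the ACBattleManager component create the battle interface, spawn the player and enemies, and resume the battle in sequence.
; Right mouse click cancels targeting through the ACTargetManager component.
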(event EventBeginPlay
  (Input|SetInputModeGameandUI self 0 "DoNotLock" false false)
  (Variables|Default|SetbShowMouseCursor true)
  (Utilities|FlowControl|Delay 0.2)
  (Utilities|FlowControl|Sequence
    (:then_0
      (Default|CreateBattleInterface (Variables|Default|GetAC_BattleManager)))
    (:then_1
      (Default|SpawnPlayerCharacter (Variables|Default|GetAC_BattleManager)))
    (:then_2
      (Default|SpawnEnemies (Variables|Default|GetAC_BattleManager)))
    (:then_3
      (Default|ResumeBattle (Variables|Default|GetAC_BattleManager)))))

(event EventTick
  (params (DeltaSeconds :type Float%20%28single-precision%29)))

(event Input|MouseEvents|RightMouseButton
  (params (Key :type Key%20Structure :default "None"))
  (:Pressed
    (Default|CancelTargeting (Variables|Default|GetAC_TargetManager))))

(fn ConstructionScript)
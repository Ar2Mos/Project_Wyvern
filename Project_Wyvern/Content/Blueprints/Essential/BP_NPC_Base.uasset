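; Base NPC Blueprint that makes an actor available for interaction with the world character.
; The construction script sizes the InteractionRange sphere from InteractionRadius.
; Overlap events on that sphere add or remove the NPC in the overlapping BP_WorldCharacter's ActorsInInteractionRange list.
; OnInteractionEnabled and OnInteractionDisabled show and hide the NPC's Widget component, with no caller for either in this Blueprint.
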(event OnComponentBeginOverlap(InteractionRange)
  (params (OverlappedComponent :type Primitive%20Component%20Object%20Reference) (OtherActor :type Actor%20Object%20Reference) (OtherComp :type Primitive%20Component%20Object%20Reference) (OtherBodyIndex :type Integer) (bFromSweep :type Boolean) (SweepResult :type Hit%20Result%20Structure%20%28by%20ref%29))
  (bind _asbp_world_character (Utilities|Casting|CastToBP_WorldCharacter OtherActor))
  (Utilities|Array|Add (Variables|/Game/Blueprints/Essential/BP_WorldCharacter.BP_WorldCharacter_C|GetActorsInInteractionRange _asbp_world_character) self))

(event OnComponentEndOverlap(InteractionRange)
  (params (OverlappedComponent :type Primitive%20Component%20Object%20Reference) (OtherActor :type Actor%20Object%20Reference) (OtherComp :type Primitive%20Component%20Object%20Reference) (OtherBodyIndex :type Integer))
  (bind _asbp_world_character (Utilities|Casting|CastToBP_WorldCharacter OtherActor))
  (Utilities|Array|RemoveItem (Variables|/Game/Blueprints/Essential/BP_WorldCharacter.BP_WorldCharacter_C|GetActorsInInteractionRange _asbp_world_character) self))

(event EventBeginPlay)

(event Collision|EventActorBeginOverlap
  (params (OtherActor :type Actor%20Object%20Reference)))

(event EventTick
  (params (DeltaSeconds :type Float%20%28single-precision%29)))

(event EventOnInteractionEnabled
  (Development|SetHiddeninGame (Variables|Default|GetWidget) false false))

(event EventOnInteractionDisabled
  (Development|SetHiddeninGame (Variables|Default|GetWidget) true false))

(fn ConstructionScript
  (Components|Sphere|SetSphereRadius (Variables|Default|GetInteractionRange) (Variables|Default|GetInteractionRadius) true))
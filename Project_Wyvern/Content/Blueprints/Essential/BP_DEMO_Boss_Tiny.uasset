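; BP_DEMO_Boss_Tiny is a demo boss enemy for turn-based battles, driven by simple AI.
; On its turn it shows an attack tooltip, ends the turn, strikes a random player character using its own stats with sound and hit effect, then resumes the battle.
; On death it runs parent logic and increments the game instance's current floor; a roguelike widget popup is left disconnected.
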(event EventPerformActionbyAI
  (bind _battlemanagerreference (Variables|Default|GetBattleManagerReference))
  (bind _ac_character_battlestats (Variables|Default|GetAC_Character_BattleStats))
  (bind _battlemanagerreference_2 (Variables|Default|GetBattleManagerReference))
  (bind _playercharacters (Variables|/Game/Blueprints/Components/AC_BattleManager.AC_BattleManager_C|GetPlayerCharacters _battlemanagerreference))
  (bind _character_stats (Variables|/Game/Blueprints/Components/AC_Character_BattleStats.AC_Character_BattleStats_C|GetCharacter%20Stats _ac_character_battlestats))
  (Default|ShowBattleToolTip _battlemanagerreference_2 (Utilities|Text|FormatText "{name} attacks" (Variables|/Game/Blueprints/Components/AC_Character_BattleStats.AC_Character_BattleStats_C|GetCharacter%20Display%20Name (Variables|Default|GetAC_Character_BattleStats))))
  (Default|EndCharacterTurn _battlemanagerreference_2 1e+03)
  (Utilities|FlowControl|Delay 0.25)
  (CallFunction|OnAttacking)
  (Utilities|FlowControl|Delay 0.3)
  (bind _output_get (Variables|Default|SetTargeted (Utilities|Array|Get(acopy) _playercharacters (Math|Random|RandomIntegerinRange 0 (- (Utilities|Array|Length _playercharacters) 1)))))
  (Default|ReceiveDamage (Variables|/Game/Blueprints/Essential/BP_Character_Battle_Base.BP_Character_Battle_Base_C|GetAC_Character_BattleStats _output_get) (.Value (Utilities|Map|Find _character_stats "NewEnumerator9")) (.Value (Utilities|Map|Find _character_stats "NewEnumerator8")) (.Value (Utilities|Map|Find _character_stats "NewEnumerator10")))
  (Audio|PlaySound2D "/Game/FREE_Fantasy_Music_Pack/punch-a-rock-161647.punch-a-rock-161647" 1.0 1.0 0.0 0 0)
  (Effects|SpawnEmitteratLocation "/Game/TrailPack/Particles/Cascade/Speed/Hit/P_SpeedHit.P_SpeedHit" (Transformation|GetActorLocation _output_get))
  (Variables|Default|SetAttack? false)
  (Variables|Default|SetDamage? false)
  (Utilities|FlowControl|Delay 1.0)
  (Default|ResumeBattle (Variables|Default|GetBattleManagerReference)))

(event EventOnDeath
  (|CallParentFunction)
  (bind _asbp_gi_custom (Utilities|Casting|CastToBP_GI_Custom (Game|GetGameInstance)))
  (Variables|/Game/Blueprints/Essential/BP_GI_Custom.BP_GI_Custom_C|SetCurrentFloor _asbp_gi_custom (+ (Variables|/Game/Blueprints/Essential/BP_GI_Custom.BP_GI_Custom_C|GetCurrentFloor _asbp_gi_custom) 1)))

(fn ConstructionScript
  (|CallParentFunction))

(fn GetIsAttacking
  (return (Variables|Default|GetAttack?)))

(fn GetIsDead
  (return (Variables|Default|GetDead?)))
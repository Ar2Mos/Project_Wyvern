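; BP_CharDemo_Ally is a demo ally character for a battle system, implementing death and action events.
; On death it flags itself Dead and notifies the battle manager that a player character was killed.
; Magic and move actions look up their costs in AC_ActionManager on the player controller, then deduct HP and SP through ACCharacterBattleStats.
; Attack, damage and resurrection events are empty stubs.
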(event EventBeginPlay
  (|CallParentFunction) ; This node is disabled and will not be called.\nDrag off pins to build functionality.
)

(event Collision|EventActorBeginOverlap
  (params (OtherActor :type Actor%20Object%20Reference))
  (|CallParentFunction OtherActor) ; This node is disabled and will not be called.\nDrag off pins to build functionality.
)

(event EventTick
  (params (DeltaSeconds :type Float%20%28single-precision%29))
  (|CallParentFunction DeltaSeconds) ; This node is disabled and will not be called.\nDrag off pins to build functionality.
)

(event EventOnDeath
  (Variables|Default|SetDead? true)
  (bind _battlemanagerreference (Variables|Default|GetBattleManagerReference)
    (:then
      (Default|OnPlayerCharacterKilled _battlemanagerreference self))
    (:else)))

(event EventOnDamageReceived
  (params (Damage :type Float%20%28double-precision%29) (Critical? :type Boolean)))

(event EventOnResurrected
  (params (HealAmount :type Float%20%28double-precision%29)))

(event EventExecuteMagicAction
  (params (MagicName :type Name :default "None"))
  (bind _ac_character_battlestats (Variables|Default|GetAC_Character_BattleStats))
  (bind (_costhp _costsp) (Default|GetActionCost (Actor|GetComponentbyClass (Game|GetPlayerController 0) "/Game/Blueprints/Components/AC_ActionManager.AC_ActionManager_C") MagicName))
  (Default|ReduceHP _ac_character_battlestats _costhp)
  (Default|ReduceSP _ac_character_battlestats _costsp))

(event EventExecuteMoveAction
  (params (MoveName :type Name :default "None"))
  (bind _ac_character_battlestats (Variables|Default|GetAC_Character_BattleStats))
  (bind (_costhp _costsp) (Default|GetActionCost (Actor|GetComponentbyClass (Game|GetPlayerController 0) "/Game/Blueprints/Components/AC_ActionManager.AC_ActionManager_C") MoveName))
  (Default|ReduceHP _ac_character_battlestats _costhp)
  (Default|ReduceSP _ac_character_battlestats _costsp))

(event EventExecuteAttackAction)

(fn ConstructionScript
  (|CallParentFunction))